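; A labelled trigger button that sends an overlapping character into a hosted or joined "dreamland" session, inactive in the n00dSleeperDemonstration level.
; On authority, the Open flag selects host or client.
; Hosting freezes the character, ramps vignette, then opens the target map or, at random, a nightmare map as a listen server.
; Joining opens the target IP immediately while a timeline ramps post-process intensity and spawned fog.
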(event `self.Box.OnComponentBeginOverlap`
  (params (OverlappedComponent :type "PrimitiveComponent Object Reference") (OtherActor :type "Actor Object Reference") (OtherComp :type "PrimitiveComponent Object Reference") (OtherBodyIndex :type Integer) (bFromSweep :type Boolean) (SweepResult :type "HitResult Structure (by ref)"))
  (`/Engine/EditorBlueprintResources/ActorMacros.Switch Has Authority`
    (:`Authority`
      (bind _returnvalue (`GameplayStatics.GetCurrentLevelName` true))
      (if (`KismetStringLibrary.EqualEqual_StrStr` _returnvalue "n00dSleeperDemonstration")
        _
        (elif (`self.Open`)
          ;[1 1 1] Open host game
          (bind _ascharacter (cast `Character` OtherActor))
          (`CharacterMovementComponent.DisableMovement` (`Character.CharacterMovement` _ascharacter))
          (bind _returnvalue_2 (`GameplayStatics.GetActorOfClass` "/Script/Engine.PostProcessVolume"))
          (`GameplayStatics.PlaySound2D` "/Engine/EditorSounds/GamePreview/PossessPlayer_Cue.PossessPlayer_Cue" 1.0 1.0 0.0 null null)
          (bind (_direction _newtrack_0) (`Timeline|DreamlandCreateTimeline`)
            (:`Update`
              (setmembers `PostProcessSettings` :`StructRef` (`PostProcessVolume.Settings` _returnvalue_2) :`VignetteIntensity` (* _newtrack_0 20.0)))
            (:`Finished`
              (`KismetSystemLibrary.ExecuteConsoleCommand` (`KismetStringLibrary.Concat_StrStr` "open " (`KismetMathLibrary.SelectString` "n00dSleeperDemoNightmare" (`KismetStringLibrary.Conv_NameToString` (`self.ButtonTargetMap`)) (`KismetMathLibrary.RandomBool`)) "?listen") (cast `PlayerController` (`Pawn.GetController` _ascharacter) :!pure true))))
          (else
            ;[1 1 1] Open client game
            (bind _ascharacter_2 (cast `Character` OtherActor))
            (`KismetSystemLibrary.ExecuteConsoleCommand` (`KismetStringLibrary.Concat_StrStr` "open " (`KismetStringLibrary.Conv_NameToString` (`self.ButtonTargetIP`))) (cast `PlayerController` (`Pawn.GetController` _ascharacter_2) :!pure true))
            (bind _returnvalue_3 (`GameplayStatics.GetActorOfClass` "/Script/Engine.PostProcessVolume"))
            (bind _returnvalue_4 (`|SpawnActorFromClass` "/Script/Engine.ExponentialHeightFog" (`KismetMathLibrary.MakeTransform` (0.0 0.0 0.0)) "Undefined" "OverrideRootScale" null null))
            (`GameplayStatics.PlaySound2D` "/n00dSleeper/Testing/Audio/A_Warp_Cue.A_Warp_Cue" 1.0 1.0 0.0 null null)
            (bind (_direction_2 _newtrack_0_2) (`Timeline|DreamlandJoinTimeline`)
              (:`Update`
                (setmembers `PostProcessSettings` :`StructRef` (`PostProcessVolume.Settings` _returnvalue_3) :`SceneFringeIntensity` (* _newtrack_0_2 20.0))
                (`ExponentialHeightFogComponent.SetFogDensity` (`ExponentialHeightFog.Component` _returnvalue_4) (/ _newtrack_0_2 10.0))))))))))

(fn `UserConstructionScript`
  (`TextRenderComponent.K2_SetText` (`self.TextRender`) (`self.ButtonName`))
  (`BillboardComponent.SetSprite` (`self.Billboard`) (`self.New Sprite`)))