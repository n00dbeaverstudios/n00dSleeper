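; Temporary pawn that stands in for a sleeper actor while its player wakes up, allowing mouse look.
; It copies the sleeper's meshes, materials and health, async-loads the wake animation, then destroys that actor.
; A MeshesBuilt RepNotify applies the appearance.
; Waking runs on spawn or on a server-routed click, multicasting the animation with a timer to spawn and possess the default pawn, passing on meshes and materials.
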(event `InputAxis|Turn`
  (params (AxisValue :type "Float (single-precision)"))
  ;[1 1 1] Mouse axis
  (`self.AddControllerYawInput` AxisValue))

(event `Key|LeftMouseButton`
  (params (Key :type "Key Structure"))
  ;[1 1 1] Sleeper
  ;;[1 1 1] Wake up on input
  (:`Pressed`
    (`self.TriggerWake`)))

(event `InputAxis|LookUp`
  (params (AxisValue :type "Float (single-precision)"))
  ;[1 1 1] Mouse axis
  (`self.AddControllerPitchInput` AxisValue))

(event `self.LoadAnimations`
  (bind _owningsleeperactor (`self.OwningSleeperActor`))
  ;[1 1 1] Load the from sleep animation from the controller settings and wake if we are waking up instantly
  (bind _sleepersettings (message `N00dSleeperInterface.N00dGetSleeperSettings` (`self.OwningController`)))
  (bind _object (`|LoadAsset` (`.FromSleep` (break `N00dSleeperAnimations` (`N00dSleeperSettings.Animations` _sleepersettings))))
    (:`Completed`
      (bind _asanim_sequence (cast `AnimSequence` _object))
      (set `self.LoadedFromSleepAnimation` _asanim_sequence)
      ;;[1 1 1] Wake up on spawn, if desired, and destroy the sleeper actor
      (if (not (`N00dSleeperSettings.WaitForPlayerInput` _sleepersettings))
        (`self.Wake`))
      (message `N00dSleeperInterface.N00dRemoveSleeper` (`GameplayStatics.GetGameMode`) _owningsleeperactor)
      (`self.K2_DestroyActor` _owningsleeperactor))))

(event `self.OnWoke`
  ;[1 1 1] Destroy self once we have woken up and created the player
  (bind _returnvalue (`self.SpawnDefaultPawn`))
  (if _returnvalue
    (`self.K2_DestroyActor`)))

(fn `ApplyMeshes`
  (returns (ReturnValue :type Boolean))
  (locals (ElementsToAdd :type Integer) (CurrentMaterialCount :type Integer))
  (bind _currentmaterialcount (`local.CurrentMaterialCount`))
  ;[1 1 1] Handle applying the meshes
  ;;[1 1 1] Get the actor components and apply the meshes over the network from the cache
  (`SkeletalMeshComponent.SetAnimation` (`self.SleeperMesh`) (`self.SleeperLoop`))
  (for (_array_element _array_index) (`self.GetSleeperMeshes`)
    (`SkinnedMeshComponent.SetSkinnedAssetAndUpdate` _array_element (`|GetArrayItem` (`self.SleeperMeshes`) _array_index) true)
    ;;[1 1 1] Apply the materials back to this mesh component
    (for _index (range _currentmaterialcount (+ _currentmaterialcount (`PrimitiveComponent.GetNumMaterials` _array_element)))
      (`self.MulticastApplyMaterials` _array_element _index (`|GetArrayItem` (`self.SleeperMaterials`) _index))
      (set `local.ElementsToAdd` _index))
    (set `local.CurrentMaterialCount` (+ (`local.ElementsToAdd`) (`local.ElementsToAdd`))))
  (return true))

(fn `GetSleeperMeshes`
  (returns (ReturnValue :type "Array of SkeletalMeshComponent Object Reference"))
  (return (`|MakeArray` (`self.SleeperMesh`))))

(fn `GiveDataToOwner`
  (returns (ReturnValue :type Boolean))
  ;[1 1 1] Give anything to the owner - this is where we may remove inventory items / health / etc and reinstate it on the player who owned it
  (return true))

(fn `InitialiseSleeperPawn`
  (params (ForController :type "PlayerController Object Reference") (OwningSleeper :type "N00dSleeperActor Object Reference"))
  (returns (ReturnValue :type Boolean))
  ;[1 1 1] Set the owner for data acquisition
  (`self.SetOwningController` ForController)
  (`self.SetOwningSleeperActor` OwningSleeper)
  ;[1 1 1] Set the parameters we care about from the actor and load and apply animations, meshes, and materials.
  (`self.GiveDataToOwner`) ; Give anything we want our owner to know about, \nback the the controller.
  (`self.LoadSleeperData`) ; Load the data off the actor onto the pawn
  (`self.LoadAnimations`) ; Load the animations from soft references
  (set `self.MeshesBuilt` true) ; Secret sauce
  (return true))

(fn `LoadSleeperData`
  (returns (ReturnValue :type Boolean))
  (bind _owningsleeperactor (`self.OwningSleeperActor`))
  ;[1 1 1] Load active references from the sleeper actor onto this pawn prior to destroying the sleeper actor
  (`self.SetSleeperPawnParams` (`N00dSleeperActor.CachedMeshes` _owningsleeperactor) (`N00dSleeperActor.CachedMaterials` _owningsleeperactor) (`N00dSleeperActor.LoadedSleepLoopAnimation` _owningsleeperactor))
  (`self.SetHealth` (`N00dSleeperActor.Health` _owningsleeperactor))
  (`self.SetMaxHealth` (`N00dSleeperActor.MaxHealth` _owningsleeperactor))
  (return false))

(fn `OnRep_MeshesBuilt`
  ;[1 1 1] Apply the meshes when relevant
  (`self.ApplyMeshes`)
  (return))

(fn `SpawnDefaultPawn`
  (returns (ReturnValue :type Boolean))
  (bind _returnvalue (`GameplayStatics.GetGameMode`))
  ;[1 1 1] Spawn and possess the default game mode pawn
  (bind _returnvalue_2 (`|SpawnActorFromClass` (`GameModeBase.DefaultPawnClass` _returnvalue) (`self.GetTransform`) "Undefined" "OverrideRootScale" _returnvalue null))
  (message `N00dSleeperInterface.N00dBuildCharacterFromSleeper` _returnvalue_2 (`self.SleeperMeshes`) (`self.SleeperMaterials`))
  (`Controller.Possess` (`self.OwningController`) _returnvalue_2)
  (return true))

(fn `ToWoke`
  (returns (ReturnValue :type Boolean))
  (bind _loadedfromsleepanimation (`self.LoadedFromSleepAnimation`))
  ;[1 1 1] Handle waking up
  (`self.MulticastSleeperAnimation` (`self.SleeperMesh`) _loadedfromsleepanimation)
  (`KismetSystemLibrary.K2_SetTimerDelegate` (`|CreateDelegate` :!event `OnWoke`) (`AnimSequenceBase.SequenceLength` _loadedfromsleepanimation))
  (return false))

(fn `TriggerWake`
  (returns (ReturnValue :type Boolean))
  ;[1 1 1] Trigger the waking process on the server only and only id we aren't already triggered
  (if (`self.Triggered`)
    _
    (elif (`self.HasAuthority` (`self.OwningController`))
      (`self.ToWoke`)
      (set `self.Triggered` true)
      (return false)
      (else
        (`self.ServerTriggerWake`))))
  (return false))

(fn `UserConstructionScript`)

(fn `Wake`
  (returns (ReturnValue :type Boolean))
  (bind _loadedfromsleepanimation (`self.LoadedFromSleepAnimation`))
  ;[1 1 1] Cast the animation to all clients and set a timer on the server for the end
  (`self.MulticastSleeperAnimation` (`self.SleeperMesh`) _loadedfromsleepanimation)
  (`KismetSystemLibrary.K2_SetTimerDelegate` (`|CreateDelegate` :!event `OnWoke`) (`AnimSequenceBase.SequenceLength` _loadedfromsleepanimation))
  (return true))