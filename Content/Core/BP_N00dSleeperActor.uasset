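; Sleeper actor that stands in for a logging-out player, copying their name, health, meshes and materials from the owning controller.
; RepNotifies trigger multicasts for appearance, widget text and the sleep loop, with animations async-loaded from the controller's sleeper settings.
; An optional proximity sphere toggles the health widget for overlapping characters.
; Interface damage reduces health until death, optionally broadcast through the game mode, then destroys the actor, optionally delayed.
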(event `self.DeathOnDelay`
  ;[1 1 1] Death on delay
  (`KismetSystemLibrary.Delay` (`self.DeathDelay`))
  (`self.K2_DestroyActor`))

(event `self.LoadAnimations`
  ;[1 1 1] Load the animations from the controller and play ToSleep
  (bind _sleepersettings (message `N00dSleeperInterface.N00dGetSleeperSettings` (`self.OwningController`)))
  (bind (_animations_tosleep _animations_sleeploop _animations_fromsleep _animations_sleephit _animations_sleepdeath) (break `N00dSleeperAnimations` (`N00dSettingsSleeper.Animations` _sleepersettings)))
  (bind _object (`|LoadAsset` _animations_tosleep)
    (:`then`
      ;;[1 1 1] Go ahead and load the other animations we need to use
      (`|ExecutionSequence`
        (:`then_0`
          (bind _object_2 (`|LoadAsset` _animations_sleeploop)
            (:`Completed`
              (bind _asanim_sequence (cast `AnimSequence` _object_2))
              (set `self.LoadedSleepLoopAnimation` _asanim_sequence))))
        (:`then_1`
          (bind _object_3 (`|LoadAsset` _animations_sleephit)
            (:`Completed`
              (bind _asanim_sequence_2 (cast `AnimSequence` _object_3))
              (set `self.LoadedHitAnimation` _asanim_sequence_2))))
        (:`then_2`
          (bind _object_4 (`|LoadAsset` _animations_sleepdeath)
            (:`Completed`
              (bind _asanim_sequence_3 (cast `AnimSequence` _object_4))
              (set `self.LoadedDeathAnimation` _asanim_sequence_3))))))
    (:`Completed`
      ;;[1 1 1] Call OnSleep once loaded
      (bind _asanim_sequence_4 (cast `AnimSequence` _object))
      (set `self.LoadedToSleepAnimation` _asanim_sequence_4)
      (`self.OnSleep`))))

(event `self.ToLoop`
  ;[1 1 1] A non-relevant function for handling anything before marking the loop as relevant
  (set `self.IsAsleep` true)
  (`self.BroadcastSleep`))

(event `self.Proximity.OnComponentBeginOverlap`
  (params (OverlappedComponent :type "PrimitiveComponent Object Reference") (OtherActor :type "Actor Object Reference") (OtherComp :type "PrimitiveComponent Object Reference") (OtherBodyIndex :type Integer) (bFromSweep :type Boolean) (SweepResult :type "HitResult Structure (by ref)"))
  ;[1 1 1] Handle overlapping
  (`self.SleeperOverlap` true OtherActor))

(event `self.Proximity.OnComponentEndOverlap`
  (params (OverlappedComponent :type "PrimitiveComponent Object Reference") (OtherActor :type "Actor Object Reference") (OtherComp :type "PrimitiveComponent Object Reference") (OtherBodyIndex :type Integer))
  ;[1 1 1] Handle overlapping
  (`self.SleeperOverlap` false OtherActor))

(event `MulticastSetHealthDisplay`
  (params (HealthToDisplay :type Text))
  ;[1 1 1] Cast the UMG changes to all clients
  (message `N00dSleeperInterfaceUMG.N00dSetSleeperHealthDisplay` (`WidgetComponent.GetUserWidgetObject` (`self.Widget`)) HealthToDisplay))

(event `MulticastSetTitleDisplay`
  (params (TitleToDisplay :type Text))
  ;[1 1 1] Cast the UMG changes to all clients
  (message `N00dSleeperInterfaceUMG.N00dSetSleeperTitleDisplay` (`WidgetComponent.GetUserWidgetObject` (`self.Widget`)) TitleToDisplay))

(event `N00dSleeperInterface.N00dSleeperDamage`
  (params (ByAmount :type "Float (single-precision)") (Instigator :type "Controller Object Reference") (Causer :type "Actor Object Reference") (DamageType :type "DamageType Class Reference"))
  ;[1 1 1] Receive damage and process it
  (`self.DamageSleeper` ByAmount Instigator Causer DamageType))

(fn `ApplyMeshes`
  (returns (ReturnValue :type Boolean))
  (locals (ElementsToAdd :type Integer) (CurrentMaterialCount :type Integer))
  (bind _currentmaterialcount (`local.CurrentMaterialCount`))
  ;[1 1 1] Handle applying the meshes
  ;;[1 1 1] Get the actor components and apply the meshes over the network from the cache
  (for (_array_element _array_index) (`self.GetSleeperMeshes`)
    (`self.MulticastApplyMeshes` _array_element (`|GetArrayItem` (`self.CachedMeshes`) _array_index))
    ;;[1 1 1] Apply the materials back to this mesh component
    (for _index (range _currentmaterialcount (+ _currentmaterialcount (`PrimitiveComponent.GetNumMaterials` _array_element)))
      (`self.MulticastApplyMaterials` _array_element _index (`|GetArrayItem` (`self.CachedMaterials`) _index))
      (set `local.ElementsToAdd` _index))
    (set `local.CurrentMaterialCount` (+ (`local.ElementsToAdd`) (`local.ElementsToAdd`))))
  (return true))

(fn `BroadcastDeath`
  (returns (ReturnValue :type Boolean))
  (if (`self.ShouldBroadcastDeath`)
    ;[1 1 1] Get the name of the player who killed the sleeper and the weapon, and broadcast that to the server
    (bind _data (message `N00dSleeperInterface.N00dSleeperGetData` (`self.DamageInstigator`)))
    (message `N00dSleeperInterface.N00dSleeperBroadcastMessage` (`GameplayStatics.GetGameMode`) (`|FormatText` "{Player} Died {Killed}" (`self.SleeperName`) (`|FormatText` "Killed by {Player} with their {Weapon}" (`.Name` (break `N00dSleeperPlayerData` (`.PlayerData` (break `N00dSleeperData` _data)))) (`KismetSystemLibrary.GetDisplayName` (`self.DamageCauser`)))))
    (return true)
    (else
      (return false))))

(fn `BroadcastSleep`
  (returns (ReturnValue :type Boolean))
  (if (`self.ShouldBroadcastSleep`)
    (message `N00dSleeperInterface.N00dSleeperBroadcastMessage` (`GameplayStatics.GetGameMode`) (`|FormatText` "{Player} is now Asleep" (`self.SleeperName`)))
    (return true)
    (else
      (return false))))

(fn `CacheMaterials`
  (params (Material :type "MaterialInterface Object Reference") (OnIndex :type Integer))
  (returns (ReturnValue :type Boolean))
  (`KismetArrayLibrary.Array_Set` (`self.CachedMaterials`) OnIndex Material true)
  (return true))

(fn `CacheMeshes`
  (params (Mesh :type "SkeletalMesh Object Reference") (OnIndex :type Integer))
  (returns (ReturnValue :type Boolean))
  ;[1 1 1] Cache the meshes on the specified index
  (`KismetArrayLibrary.Array_Set` (`self.CachedMeshes`) OnIndex Mesh true)
  (return true))

(fn `DamageSleeper`
  (params (DamageAmount :type "Float (double-precision)") (DInstigator :type "Controller Object Reference") (DCauser :type "Actor Object Reference") (DamageTypeClass :type "DamageType Class Reference"))
  (returns (ReturnValue :type Boolean))
  ;[1 1 1] Damage
  (bind _output_get (set `self.DamageInstigator` DInstigator))
  (bind _output_get_2 (set `self.DamageCauser` DCauser))
  (bind _returnvalue (`GameplayStatics.ApplyDamage` self DamageAmount _output_get _output_get_2 DamageTypeClass))
  (`self.ModifyHealth` _returnvalue)
  (return false))

(fn `FormatHealth`
  (params (CurrentHealth :type "Float (double-precision)"))
  (returns (Formatted :type Text))
  ;[1 1 1] Convert health & max health to formatted text
  (return (`|FormatText` "{Current} / {Max}" (`KismetMathLibrary.Round` CurrentHealth) (`KismetMathLibrary.Round` (`self.MaxHealth`)))))

(fn `GetSleeperMeshes`
  (returns (ReturnValue :type "Array of SkeletalMeshComponent Object Reference"))
  (return (`|MakeArray` (`self.SleeperMesh`))))

(fn `InitialiseSleeper`
  (params (ForController :type "PlayerController Object Reference"))
  (returns (ReturnValue :type Boolean))
  (locals (LocalMeshes :type "Array of SkeletalMesh Object Reference") (LocalController :type "PlayerController Object Reference") (LocalMaterials :type "Array of MaterialInterface Object Reference") (LocalAnimInstance :type "AnimInstance Class Reference"))
  ;[1 1 1] Initialise the sleeper actor when spawned
  (`self.SetOwningController` ForController)
  ;;[1 1 1] Cache this sleeper on the Game Mode
  (message `N00dSleeperInterface.N00dAddSleeper` (`GameplayStatics.GetGameMode`) self)
  ;;[1 1 1] Setup the owner
  (bind _returnvalue (`self.SetupSleeperFromOwnerData`))
  (return _returnvalue))

(fn `KillSleeper`
  (returns (ReturnValue :type Boolean))
  ;[1 1 1] Kill the sleeper according to our conditions
  (`KismetSystemLibrary.PrintString` "Sleeper Dead")
  (`self.BroadcastDeath`)
  (set `self.HealthDisplay` "DEAD")
  (set `self.Dead` true)
  (`self.OnSleeperDead` (`self.SleeperOwnerID`))
  (if (> (`self.DeathDelay`) 0.0)
    (`self.DeathOnDelay`)
    (else
      (`self.K2_DestroyActor`)))
  (return false))

(fn `ModifyHealth`
  (params (DamageIn :type "Float (double-precision)"))
  (returns (ReturnValue :type Boolean))
  ;[1 1 1] Set the new health minus the damage and process it for displaying on the widget if valid
  ;;[1 1 1] Feed in the modified value to the set health function, and if the function returns true, kill.
  (bind (_isdead _outhealth) (`self.SetHealth` (- (`self.Health`) DamageIn)))
  (if _isdead
    ;;[1 1 1] Kill or return for more torture
    (`self.KillSleeper`)
    (else
      (set `self.HealthDisplay` (`self.FormatHealth` _outhealth))
      (`self.SleeperHit`)))
  (return true))

(fn `N00dGetIsSleeperDead`
  (returns (IsDead :type Boolean))
  (return (`self.Dead`)))

(fn `N00dGetSleeperID`
  (returns (SleeperID :type String))
  (return ""))

(fn `N00dGetSleeperSettings`
  (returns (SleeperSettings :type "N00dSettingsSleeper Object Reference") (SaveGame :type "SaveGame Object Reference"))
  (return null null))

(fn `N00dSleeperGetData`
  (returns (Data :type "N00dSleeperData Structure"))
  (return))

(fn `OnRep_Dead`
  (return))

(fn `OnRep_HealthDisplay`
  (`self.MulticastSetHealthDisplay` (`self.HealthDisplay`))
  (return))

(fn `OnRep_IsAsleep`
  ;[1 1 1] Perform the IsAsleep OnRep when relevant
  (if (`self.IsAsleep`)
    (`self.MulticastSleeperAnimation` (`self.SleeperMesh`) (`self.LoadedSleepLoopAnimation`) true)
    (`self.MulticastSetSphereRadius` (`self.Proximity`) (`self.ProximityRadius`)))
  (return))

(fn `OnRep_MeshesBuilt`
  ;[1 1 1] When relevant, reapply the meshes
  (`self.ApplyMeshes`)
  (return))

(fn `OnRep_TitleName`
  (`self.MulticastSetTitleDisplay` (`self.TitleName`))
  (return))

(fn `OnSleep`
  (returns (ReturnValue :type Boolean))
  (bind _loadedtosleepanimation (`self.LoadedToSleepAnimation`))
  ;[1 1 1] Multicast the ToSleep animation and set a timer for when the sequence is complete
  (`self.MulticastSleeperAnimation` (`self.SleeperMesh`) _loadedtosleepanimation)
  (`KismetSystemLibrary.K2_SetTimerDelegate` (`|CreateDelegate` :!event `ToLoop`) (`AnimSequenceBase.SequenceLength` _loadedtosleepanimation))
  (return false))

(fn `SetHealth`
  (params (NewHealth :type "Float (double-precision)"))
  (returns (IsDead :type Boolean) (OutHealth :type "Float (double-precision)"))
  (bind _output_get (set `self.Health` NewHealth))
  (return (<= _output_get 0.0) _output_get))

(fn `SetupProximity`
  (returns (ReturnValue :type Boolean))
  (bind _proximity (`self.Proximity`))
  ;[1 1 1] Construct the proxy if required
  (if (`self.UseProximity`)
    ;;[1 1 1] Proxy
    (`PrimitiveComponent.SetCollisionEnabled` _proximity "QueryOnly")
    (`SphereComponent.SetSphereRadius` _proximity (`self.ProximityRadius`) true)
    (return true)
    (else
      (return false))))

(fn `SetupSleeperFromOwnerData`
  (returns (ReturnValue :type Boolean))
  (locals (LocalMeshes :type "Array of SkeletalMesh Object Reference") (LocalMaterials :type "Array of MaterialInterface Object Reference"))
  ;[1 1 1] While we are logging out, grab what we need from the controller and apply it to this actor
  ;;[1 1 1] Set the owner ID on this actor from the controller
  (bind _sleeperid (message `N00dSleeperInterface.N00dGetSleeperID` (`self.OwningController`)))
  (`self.SetOwnerID` _sleeperid)
  ;;[1 1 1] Load the meshes and set the player data
  (bind _data (message `N00dSleeperInterface.N00dSleeperGetData` (`self.OwningController`)))
  (set `local.LocalMeshes` (`.Meshes` (break `N00dSleeperData` _data)))
  (set `local.LocalMaterials` (`.Materials` (break `N00dSleeperData` _data)))
  (bind (_name _healthcurrent _healthmax) (break `N00dSleeperPlayerData` (break `N00dSleeperData` _data)))
  (`self.SetOwnerName` _name)
  (`self.SetHealth` _healthcurrent)
  (`self.SetMaxHealth` _healthmax)
  ;;[1 1 1] Setup the widget
  (`self.SetupWidget`)
  ;;[1 1 1] Get the sleeper settings that are relevant to this actor
  (bind (_sleepersettings _savegame) (message `N00dSleeperInterface.N00dGetSleeperSettings` (`self.OwningController`)))
  (if (`N00dSettingsSleeper.ShouldBroadcastSleep` _sleepersettings)
    (`self.BroadcastSleep`))
  (`self.SetSleeperActorParameters` (`N00dSettingsSleeper.ShouldBroadcastDeath` _sleepersettings) (`N00dSettingsSleeper.DeathDelay` _sleepersettings) (`N00dSettingsSleeper.UseProximity` _sleepersettings) (`N00dSettingsSleeper.ProximityRadius` _sleepersettings) (`N00dSettingsSleeper.ShowWidgetOnSleeperDamage` _sleepersettings) (`N00dSettingsSleeper.SleeperWidgetCloseDelay` _sleepersettings) _savegame (`N00dSettingsSleeper.SleeperSaveSlot` _sleepersettings))
  (`self.SetupProximity`)
  ;;[1 1 1] Cache the meshes
  (for (_ _array_index) (`self.GetSleeperMeshes`)
    (`self.CacheMeshes` (`|GetArrayItem` (`local.LocalMeshes`) _array_index) _array_index))
  (for (_array_element _array_index_2) (`local.LocalMaterials`)
    (`self.CacheMaterials` _array_element _array_index_2))
  ;;[1 1 1] Finally
  ;;;[1 1 1] Load animations
  (`self.LoadAnimations`)
  ;;;[1 1 1] Notify of the relevancy
  (bind _output_get (set `self.MeshesBuilt` true)) ; Magic sauce
  (return _output_get))

(fn `SetupWidget`
  (returns (ReturnValue :type Boolean))
  ;[1 1 1] If the widget exists, get the player data and set the relevant values that we care about over the network so everyone can see.
  (`/Engine/EditorBlueprintResources/StandardMacros.IsValid` (`WidgetComponent.GetUserWidgetObject` (`self.Widget`))
    (:`Is Valid`
      (bind _data (message `N00dSleeperInterface.N00dSleeperGetData` (`self.OwningController`)))
      (bind ((`Name` _name) (`HealthCurrent` _healthcurrent)) (break `N00dSleeperPlayerData` (`.PlayerData` (break `N00dSleeperData` _data))))
      (set `self.TitleName` _name)
      (set `self.HealthDisplay` (`self.FormatHealth` _healthcurrent))
      (return true))
    (:`Is Not Valid`
      (return false))))

(fn `SleeperHit`
  (returns (ReturnValue :type Boolean))
  ;[1 1 1] Have custom stuff happen when the sleeper is damaged
  (return false))

(fn `SleeperOverlap`
  (params (Begin :type Boolean) (OtherActor :type "Actor Object Reference"))
  (returns (ReturnValue :type Boolean))
  (locals (LocalController :type "Controller Object Reference") (LocalCharacter :type "Character Object Reference"))
  ;[1 1 1] Handle Overlap
  ;;[1 1 1] Cache the controller over the overlapper as a local for cleanliness
  (if (`self.UseProximity`)
    (bind _ascharacter (cast `Character` OtherActor)
      (:`then`
        (bind _output_get (set `local.LocalCharacter` _ascharacter))
        (set `local.LocalController` (`Pawn.GetController` _output_get))
        (if Begin
          ;;[1 1 1] Add the overlapped player to the proxies
          (message `N00dSleeperInterface.N00dSleeperWidgetVisibility` (`local.LocalController`) (`self.Widget`) true)
          (`self.AddPlayerToProxies` (`local.LocalCharacter`))
          (else
            ;;[1 1 1] Remove the player from the stack and stop displaying the widget
            (`self.RemovePlayerFromProxies` (`local.LocalCharacter`))
            (message `N00dSleeperInterface.N00dSleeperWidgetVisibility` (`local.LocalController`) (`self.Widget`) false)))
        (return false))
      (:`CastFailed`
        (return false)))
    (else
      (return false))))

(fn `UserConstructionScript`)