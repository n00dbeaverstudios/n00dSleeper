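; Sleeper component that leaves a sleeper actor in place of a logged-out player and respawns the returning player there.
; Logout captures meshes and materials into controller data, then spawns the controller's configured sleeper actor.
; Respawn matches cached sleepers by player ID, checking death rules before spawning the sleeper pawn or default pawn.
; In-game sleep/wake disables movement, async-loads animations and multicasts them on timers; overridable hooks allow custom rules.
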(event `self.BuildCharacterMeshComponents`
  (params (SkeletalComponents :type "Array of SkeletalMeshComponent Object Reference (by ref)"))
  (bind _returnvalue (`Pawn.GetController` (`self.OwningCharacter`)))
  ;[1 1 1] Build the character mesh components
  ;;[1 1 1] Set a reference to the components
  (set `self.MeshComponents` SkeletalComponents)
  ;;[1 1 1] Unpack the skeletal meshes from the components into the stack
  (for (_array_element _array_index) (`self.MeshComponents`)
    (`KismetArrayLibrary.Array_Set` (`self.CharacterMeshes`) _array_index (`SkinnedMeshComponent.SkeletalMesh` _array_element) true))
  ;;[1 1 1] Set the mesh array on the controller
  (bind _data (message `N00dSleeperInterface.N00dSleeperGetData` _returnvalue))
  (bind _structout (setmembers `N00dSleeperData` :`StructRef` _data :`Meshes` (`self.CharacterMeshes`)))
  (message `N00dSleeperInterface.N00dSleeperSetData` _returnvalue _structout))

(event `self.LoadSleepAnimations`
  ;[1 1 1] Load the animations if we are triggered
  (bind _sleepersettings (message `N00dSleeperInterface.N00dGetSleeperSettings` (`self.OwningController`)))
  (bind ((`ToSleep` _tosleep) (`SleepLoop` _sleeploop) (`FromSleep` _fromsleep)) (break `N00dSleeperAnimations` (`N00dSettingsSleeper.Animations` _sleepersettings)))
  (bind _object (`|LoadAsset` _tosleep)
    (:`Completed`
      (bind _asanim_sequence (cast `AnimSequence` _object))
      (set `self.LoadedToSleep` _asanim_sequence)
      (`self.OnSleep`)
      (bind _object_2 (`|LoadAsset` _sleeploop)
        (:`Completed`
          (bind _asanim_sequence_2 (cast `AnimSequence` _object_2))
          (set `self.LoadedSleepLoop` _asanim_sequence_2)
          (bind _object_3 (`|LoadAsset` _fromsleep)
            (:`Completed`
              (bind _asanim_sequence_3 (cast `AnimSequence` _object_3))
              (set `self.LoadedFromSleep` _asanim_sequence_3))))))))

(event `self.ToLoop`
  (bind _owningcontroller (`self.OwningController`))
  ;[1 1 1] Disable movement and flag us as asleep
  (`self.MulticastSleepAnimation` (`Character.Mesh` (`self.OwningCharacter`)) (`self.LoadedSleepLoop`))
  (set `self.Asleep` true)
  (set `self.Triggered` false)
  ;[1 1 1] Broadcast the sleeper message if required
  (bind _sleepersettings (message `N00dSleeperInterface.N00dGetSleeperSettings` _owningcontroller))
  (if (`N00dSettingsSleeper.ShouldBroadcastSleep` _sleepersettings)
    (bind _data (message `N00dSleeperInterface.N00dSleeperGetData` _owningcontroller))
    (message `N00dSleeperInterface.N00dSleeperBroadcastMessage` (`GameplayStatics.GetGameMode`) (`|FormatText` "{Player} is now Asleep" (`.Name` (break `N00dSleeperPlayerData` (`.PlayerData` (break `N00dSleeperData` _data))))))))

(event `self.ToWoke`
  (bind _owningcharacter (`self.OwningCharacter`))
  ;[1 1 1] Reinstate movement and anim instance and flag us as awake
  (`CharacterMovementComponent.SetMovementMode` (`Character.CharacterMovement` _owningcharacter) "MOVE_Walking" 0)
  (set `self.Asleep` false)
  (set `self.Triggered` false)
  (`self.MulticastSetAnimInstance` (`Character.Mesh` _owningcharacter)))

(fn `AddSleeper`
  (params (SleeperActor :type "N00dSleeperActor Object Reference"))
  (returns (ReturnValue :type Boolean))
  ;[1 1 1] Add sleeper to cache
  (`KismetArrayLibrary.Array_Add` (`self.SleeperCache`) SleeperActor)
  (return true))

(fn `ApplyMeshes`
  (returns (ReturnValue :type Boolean))
  (locals (CurrentMaterialCount :type Integer) (ElementsToAdd :type Integer))
  (bind _currentmaterialcount (`local.CurrentMaterialCount`))
  ;[1 1 1] Handle applying the meshes
  ;;[1 1 1] Get the actor components and apply the meshes over the network from the cache
  (for (_array_element _array_index) (`self.MeshComponents`)
    (`SkinnedMeshComponent.SetSkinnedAssetAndUpdate` _array_element (`|GetArrayItem` (`self.CharacterMeshes`) _array_index) true)
    ;;[1 1 1] Apply the materials back to this mesh component
    (for _index (range _currentmaterialcount (+ _currentmaterialcount (`PrimitiveComponent.GetNumMaterials` _array_element)))
      (`PrimitiveComponent.SetMaterial` _array_element _index (`|GetArrayItem` (`self.CharacterMaterials`) _index))
      (set `local.ElementsToAdd` _index))
    (set `local.CurrentMaterialCount` (+ (`local.ElementsToAdd`) (`local.ElementsToAdd`))))
  (return true))

(fn `BroadcastSleeperMessage`
  (params (Message :type "Text (by ref)"))
  (returns (ReturnValue :type Boolean))
  ;[1 1 1] Handle this however you choose - ideally with an interface that talks to your HUD and Text within as the PlayerCache consists of all the active player controllers that exist on the server (could also Cast if you want)
  (for _ (`self.PlayerCache`)
    (`KismetSystemLibrary.PrintString` (`KismetTextLibrary.Conv_TextToString` Message)))
  (return false))

(fn `CanSleep`
  (returns (ReturnValue :type Boolean))
  ;[1 1 1] Override to handle any custom conditions
  (return true))

(fn `CanSpawnAtSleeper`
  (params (ForController :type "PlayerController Object Reference") (Sleeper :type "N00dSleeperActor Object Reference"))
  (returns (ReturnValue :type Boolean))
  (locals (LocalSleeper :type "N00dSleeperActor Object Reference"))
  ;[1 1 1] Cache the settings and sleeper
  (set `local.LocalSleeper` Sleeper)
  (bind _sleepersettings (message `N00dSleeperInterface.N00dGetSleeperSettings` ForController))
  ;[1 1 1] Did we find a sleeper, if not, return false to spawn default
  (`/Engine/EditorBlueprintResources/StandardMacros.IsValid` (`local.LocalSleeper`)
    (:`Is Valid`
      ;[1 1 1] Is the sleeper dead, if not we can spawn
      (bind _isdead (message `N00dSleeperInterface.N00dGetIsSleeperDead` (`local.LocalSleeper`)))
      (if _isdead
        ;[1 1 1] Are we spawning at the sleeper even if we have died, return true if we can, false will spawn default pawn
        (if (`N00dSettingsSleeper.SpawnAtSleeperIfDead` _sleepersettings)
          (return true)
          (else
            (return false)))
        (else
          (return true))))
    (:`Is Not Valid`
      (return false))))

(fn `ClearSleepers`
  (returns (ReturnValue :type Boolean))
  ;[1 1 1] Clear cache
  (`KismetArrayLibrary.Array_Clear` (`self.SleeperCache`))
  (return true))

(fn `DefaultSpawn`
  (params (ForController :type "PlayerController Object Reference"))
  (returns (DefaultPawn :type "Pawn Object Reference"))
  (bind _returnvalue (`GameplayStatics.GetGameMode`))
  ;[1 1 1] Override for custom default spawn logic - this executes on initial sign in
  (bind _returnvalue_2 (`|SpawnActorFromClass` (`GameModeBase.DefaultPawnClass` _returnvalue) (`Actor.GetTransform` (`GameModeBase.K2_FindPlayerStart` _returnvalue ForController "")) "Undefined" "OverrideRootScale" null null))
  (return _returnvalue_2))

(fn `FindSleeper`
  (params (ForController :type "PlayerController Object Reference"))
  (returns (SleeperActor :type "N00dSleeperActor Object Reference") (ReturnValue :type Boolean))
  (locals (LocalFound :type Boolean) (LocalSleeper :type "N00dSleeperActor Object Reference"))
  ;[1 1 1] Loop the sleeper cache, compare with the invoking player controller, and return
  (for _array_element (`self.SleeperCache`)
    (`/Engine/EditorBlueprintResources/StandardMacros.IsValid` _array_element
      (:`Is Valid`
        (if (`KismetStringLibrary.EqualEqual_StrStr` (`self.GetSleeperPlayerID` ForController) (`N00dSleeperActor.SleeperOwnerID` _array_element))
          (set `local.LocalFound` true)
          (set `local.LocalSleeper` _array_element)))))
  (return (`local.LocalSleeper`) (`local.LocalFound`)))

(fn `GetSleeperPlayerID`
  (params (ForController :type "PlayerController Object Reference"))
  (returns (PlayerID :type String))
  ;[1 1 1] Override for your own method of ID acquisition
  (return (`PlayerState.GetPlayerName` (`Controller.PlayerState` ForController))))

(fn `InitialiseSleeperPlayer`
  (params (Owner :type "Character Object Reference") (SkeletalComponents :type "Array of SkeletalMeshComponent Object Reference (by ref)"))
  (returns (ReturnValue :type Boolean))
  ;[1 1 1] Begin Play on the character
  ;;[1 1 1] Build references to the owning player and our relevant data
  (bind _output_get (set `self.MeshComponents` SkeletalComponents))
  (`self.BuildCharacterMeshComponents` _output_get)
  (`self.ServerSetOwningController` (cast `PlayerController` (`Pawn.GetController` Owner) :!pure true))
  (return false))

(fn `OnRep_MeshesBuilt`
  ;[1 1 1] Apply the relevant meshes
  (`self.ApplyMeshes`)
  (return))

(fn `OnSleep`
  (returns (ReturnValue :type Boolean))
  (bind _loadedtosleep (`self.LoadedToSleep`))
  (bind _mesh (`Character.Mesh` (`self.OwningCharacter`)))
  ;[1 1 1] Multicast the sleeping animation and wait for the animation to finish
  (set `self.CachedAnimInstance` (`GameplayStatics.GetObjectClass` (`SkeletalMeshComponent.GetAnimInstance` _mesh))) ; Cache the animation before playing the sleep anim
  (`self.MulticastSleepAnimation` _mesh _loadedtosleep)
  (`KismetSystemLibrary.K2_SetTimerDelegate` (`|CreateDelegate` :!event `ToLoop`) (`AnimSequenceBase.SequenceLength` _loadedtosleep))
  (return false))

(fn `RefreshOtherData`
  (returns (ReturnValue :type Boolean))
  ;[1 1 1] Override for refreshing any extra logic prior to initialising the sleeper
  (return false))

(fn `RefreshSleeperMeshes`
  (returns (ReturnValue :type Boolean))
  ;[1 1 1] Reference all the relevant meshes and their materials - this is called when logging off and will rebuild our meshes from owning mesh components
  ;;[1 1 1] Get the mesh components in memory and refresh the references to the meshes
  (for (_array_element _array_index) (`self.MeshComponents`)
    (`KismetArrayLibrary.Array_Set` (`self.CharacterMeshes`) _array_index (`SkinnedMeshComponent.SkeletalMesh` _array_element))
    ;;[1 1 1] Reference all the materials for every mesh we have
    (for _array_element_2 (`MeshComponent.GetMaterials` _array_element)
      (`self.BuildCharacterMaterials` _array_element_2)))
  (message `N00dSleeperInterface.N00dSleeperSetData` (`self.OwningController`) (make `N00dSleeperData` (struct) (`self.CharacterMeshes`) (`self.CharacterMaterials`)))
  (return true))

(fn `RemoveSleeper`
  (params (SleeperActor :type "N00dSleeperActor Object Reference"))
  (returns (ReturnValue :type Boolean))
  ;[1 1 1] Remove sleeper from cache
  (bind _returnvalue (`KismetArrayLibrary.Array_RemoveItem` (`self.SleeperCache`) SleeperActor))
  (return _returnvalue))

(fn `Respawn`
  (params (ForController :type "PlayerController Object Reference"))
  (returns (SpawnedPawn :type "Pawn Object Reference"))
  (locals (LocalSleeper :type "N00dSleeperActor Object Reference") (LocalFound :type Boolean :default false) (LocalController :type "PlayerController Object Reference"))
  (bind _localcontroller (`local.LocalController`))
  ;[1 1 1] Handle spawning at the sleeper according to our conditions
  ;;[1 1 1] Cache and find the sleeper
  (bind _output_get (set `local.LocalController` ForController))
  (bind _sleeperactor (`self.FindSleeper` _output_get))
  (set `local.LocalSleeper` _sleeperactor)
  ;;[1 1 1] Can spawn at sleeper
  (if (`self.CanSpawnAtSleeper` (`local.LocalController`) (`local.LocalSleeper`))
    ;;[1 1 1] If we find a sleeper and we can spawn, spawn at sleeper, otherwise spawn default pawn
    (bind _sleeperpawn (`self.SpawnAtSleeper` (`local.LocalSleeper`) _localcontroller))
    (return _sleeperpawn)
    (else
      (bind _defaultpawn (`self.DefaultSpawn` _localcontroller))
      (return _defaultpawn))))

(fn `Sleep`
  (params (Logout :type Boolean))
  (returns (ReturnValue :type Boolean))
  ;[1 1 1] Setup the data and spawn the sleeper
  ;;[1 1 1] Only do this on authority
  (if Logout
    (if (`self.CanSleep`)
      (if (`Actor.HasAuthority` (`self.OwningCharacter`))
        ;;[1 1 1] Update the owner meshes
        (`self.RefreshSleeperMeshes`)
        ;;[1 1 1] Refresh Other Data
        (`self.RefreshOtherData`)
        ;;[1 1 1] Spawn a sleeper actor
        (`self.SpawnSleeper`)
        (return false)
        (else
          _)))
    (elif (`self.Triggered`)
      _
      (elif (`self.Asleep`)
        (`self.ServerWake`)
        (else
          (`self.ServerSleep`)))))
  (return false))

(fn `SpawnAtSleeper`
  (params (SleeperActor :type "N00dSleeperActor Object Reference") (ForController :type "PlayerController Object Reference"))
  (returns (SleeperPawn :type "N00dSleeperPawn Object Reference"))
  (locals (LocalSleeperActor :type "N00dSleeperActor Object Reference") (LocalController :type "PlayerController Object Reference"))
  ;[1 1 1] Spawn at Sleeper Actor
  ;;[1 1 1] Cache
  (set `local.LocalSleeperActor` SleeperActor)
  (set `local.LocalController` ForController)
  (bind _sleepersettings (message `N00dSleeperInterface.N00dGetSleeperSettings` ForController))
  ;;[1 1 1] Spawn the sleeper pawn
  (bind _returnvalue (`|SpawnActorFromClass` (`N00dSettingsSleeper.SleeperPawn` _sleepersettings) (`Actor.GetTransform` (`local.LocalSleeperActor`)) "Undefined" "OverrideRootScale" null null))
  ;;[1 1 1] Initialise the sleeper pawn
  (`N00dSleeperPawn.InitialiseSleeperPawn` _returnvalue (`local.LocalController`) (`local.LocalSleeperActor`))
  (return _returnvalue))

(fn `SpawnSleeper`
  (returns (ReturnValue :type Boolean))
  ;[1 1 1] Get the sleeper actor class from the controller settings and initialise
  (bind _sleepersettings (message `N00dSleeperInterface.N00dGetSleeperSettings` (`self.OwningController`)))
  (bind _returnvalue (`|SpawnActorFromClass` (`N00dSettingsSleeper.SleeperActor` _sleepersettings) (`Actor.GetTransform` (`self.OwningCharacter`)) "Undefined" "OverrideRootScale" null null))
  (`/Engine/EditorBlueprintResources/StandardMacros.IsValid` _returnvalue
    (:`Is Valid`
      (bind _returnvalue_2 (`N00dSleeperActor.InitialiseSleeper` _returnvalue (`self.OwningController`)))
      (return _returnvalue_2))
    (:`Is Not Valid`
      (return false))))

(fn `TriggerSleep`
  (returns (ReturnValue :type Boolean))
  ;[1 1 1] Trigger the sleep by disabling the movement and load the sleep animations, and set a bool letting us know we have been triggered.
  (`CharacterMovementComponent.DisableMovement` (`Character.CharacterMovement` (`self.OwningCharacter`)))
  (set `self.Triggered` true)
  (`self.LoadSleepAnimations`)
  (return false))

(fn `TriggerWake`
  (returns (ReturnValue :type Boolean))
  (bind _loadedfromsleep (`self.LoadedFromSleep`))
  ;[1 1 1] Trigger the waking process by mulitcasting the wake animation, and setting a timer for once the animation has complete
  (set `self.Triggered` true)
  (`self.MulticastSleepAnimation` (`Character.Mesh` (`self.OwningCharacter`)) _loadedfromsleep)
  (`KismetSystemLibrary.K2_SetTimerDelegate` (`|CreateDelegate` :!event `ToWoke`) (`AnimSequenceBase.SequenceLength` _loadedfromsleep))
  (return false))