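; Controller component for the n00dSleeper system, holding a player's sleep data for the sleep actor used on logout.
; Initialisation stores the character's mesh; the local controller sends Game Instance IDs to the server for the Game Mode.
; Locally, an optional black screen fades out after a delay, timed to the wake-up animation.
; Also provides save deletion, listen-server open/connect helpers and a debug-only sleeper death notice.
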(event `DeleteClientSave`
  ;[1 0.05 0.05] Delete the sleeper saves for client and server
  (`self.DeleteSave`))

(event `DeleteAllSleeperSaves`
  ;[1 0.05 0.05] Delete the sleeper saves for client and server
  (`self.DeleteSaves`))

(event `self.Initialise`
  (params (Owning :type "/Game/n00dSleeper/Deprecated/FOwning Structure"))
  ;[1 1 1] Initialise
  (`parent.Initialise` Owning)
  (`self.InitialiseController`))

(event `ServerSetSleeperData`
  (params (SleepData :type "/Game/n00dSleeper/Core/FN00dSleeper_Data Structure"))
  ;[0.1903 0.6116 0.705] NETWORKING
  ;;[1 1 1] Set the GUID on the server so that the game mode can read it
  (`self.SetSleepData` SleepData)
  ;;;[0.2462 0.323 0.34] DEBUG
  (`self.Debug` "Loaded SleepData ID:" "NewEnumerator2" (`.OwningID_7_B372075A4A13A2336D81F6857A069E34` (break `/Game/n00dSleeper/Core/FN00dSleeper_Data` SleepData)) false true 10.0))

(event `OwningSleepDataFromServer`
  (params (SleepData :type "/Game/n00dSleeper/Core/FN00dSleeper_Data Structure"))
  ;[0.1903 0.6116 0.705] NETWORKING
  ;;[1 1 1] Set from Game Mode (server)
  ;;;[1 1 1] Owning debug sleep data
  (bind _output_get (set `self.DebugServerSleepData` SleepData))
  ;;;[0.2462 0.323 0.34] DEBUG
  (`self.Debug` "Debug Server Sleep Data GUID:" "NewEnumerator2" (`.OwningID_7_B372075A4A13A2336D81F6857A069E34` (break `/Game/n00dSleeper/Core/FN00dSleeper_Data` _output_get))))

(event `OwningSetLoadedSleepData`
  (params (SleepData :type "/Game/n00dSleeper/Core/FN00dSleeper_Data Structure"))
  ;[0.1903 0.6116 0.705] NETWORKING
  ;;[1 1 1] Set from Game Instance (client)
  (bind _output_get (set `self.LoadedSleepData` SleepData))
  ;;;[0.2462 0.323 0.34] DEBUG
  (`self.Debug` "LOADED SleepData for Controller GUID:" "NewEnumerator2" (`.OwningID_7_B372075A4A13A2336D81F6857A069E34` (break `/Game/n00dSleeper/Core/FN00dSleeper_Data` _output_get)) false true 10.0))

(fn `BindSleeperDeath`
  ;[1 1 1] Bind an event to notify the player that he has died
  (bind _gamemodesleepcomponent (message `/Game/n00dSleeper/Core/BPI_N00dSleeper.GetGameModeSleeper` (`GameplayStatics.GetGameMode`)))
  (`/Engine/EditorBlueprintResources/StandardMacros.IsValid` _gamemodesleepcomponent
    (:`Is Valid`
      (add `/Game/n00dSleeper/Core/BPC_N00dSleeper_GameMode.OnSleeperDead` _gamemodesleepcomponent (`|CreateDelegate` :!event `NotifyDeadSleeperPlayer`))
      (return))
    (:`Is Not Valid`
      (return))))

(fn `BlackenScreen`
  (params (ForController :type "Controller Object Reference"))
  (`PlayerCameraManager.SetManualCameraFade` :`self` (`PlayerController.PlayerCameraManager` (cast `PlayerController` ForController :!pure true)) :`InFadeAmount` 1.0)
  (return))

(fn `ConstuctDefaults`
  (bind (_sleepsounds_tosleep _sleepsounds_sleeploop _sleepsounds_fromsleep) (break `/Game/n00dSleeper/Core/FN00dSleeper_Sounds` (`self.SleepSounds`)))
  (bind (_sleepanimations_tosleep _sleepanimations_sleeploop _sleepanimations_fromsleep) (break `/Game/n00dSleeper/Core/FN00dSleeper_Animation` (`self.SleepAnimations`)))
  ;[1 1 1] Set the user-defined sleeping defauts for the player in the loaded sleep data
  (bind _structout (setmembers `/Game/n00dSleeper/Core/FN00dSleeper_Data` :`StructRef` (`self.LoadedSleepData`) :`Animations` (make `/Game/n00dSleeper/Core/FN00dSleeper_Animation` _sleepanimations_tosleep _sleepanimations_sleeploop _sleepanimations_fromsleep) :`Sounds` (make `/Game/n00dSleeper/Core/FN00dSleeper_Sounds` _sleepsounds_tosleep _sleepsounds_sleeploop _sleepsounds_fromsleep)))
  (set `self.LoadedSleepData` _structout)
  (return))

(fn `DeleteSave`
  ;[1 1 1] Delete the sleep data on slot
  (bind _returnvalue (`GameplayStatics.DeleteGameInSlot` "SleeperSaveClient"))
  (if _returnvalue
    (`self.Debug` "DELETED Client Save" "NewEnumerator4")
    (else
      (`self.Debug` "NOTHING TO DELETE On Client" "NewEnumerator4")))
  (return))

(fn `DeleteSaves`
  ;[1 1 1] Delete the sleep data on slot
  (`|ExecutionSequence`
    (:`then_0`
      (bind _returnvalue (`GameplayStatics.DeleteGameInSlot` "SleeperSaveClient"))
      (if _returnvalue
        (`self.Debug` "DELETED Save(s)" "NewEnumerator4" :!label _label)
        (else
          (`self.Debug` "NOTHING TO DELETE" "NewEnumerator4" :!label _label_2))))
    (:`then_1`
      (bind _returnvalue_2 (`GameplayStatics.DeleteGameInSlot` "SleeperSaveServer"))
      (if _returnvalue_2
        (goto _label)
        (else
          (goto _label_2)))))
  (return))

(fn `GetPlayerSleepData`
  (returns (ClientSleepData :type "/Game/n00dSleeper/Core/FN00dSleeper_Data Structure"))
  ;[1 1 1] We cannot componentise the Game Instance, so we are messaging your Instance for the data
  (if (`Controller.IsLocalController` (`self.OwningController`))
    (bind _sleepdata (message `/Game/n00dSleeper/Core/BPI_N00dSleeper.GetSleepData` (`GameplayStatics.GetGameInstance`)))
    (return _sleepdata) ; Let's do this
    (else
      (return) ; Forget about it
    )))

(fn `InitialiseController`
  ;[1 1 1] Save the parent mesh of the owning character in the controller's loaded sleep data, to use on the sleep actor on logout
  (bind _structout (setmembers `/Game/n00dSleeper/Core/FN00dSleeper_Data` :`StructRef` (`self.LoadedSleepData`) :`SkeletalMesh` (`SkinnedMeshComponent.SkeletalMesh` (`self.OwningSkeletalMesh`))))
  (`self.SetSleepData` _structout)
  ;[1 1 1] Only do the following for the local
  (if (`Controller.IsLocalController` (`self.OwningController`))
    ;[1 1 1] Send the client IDs to the server
    (bind _sleepdata (message `/Game/n00dSleeper/Core/BPI_N00dSleeper.GetSleepData` (`GameplayStatics.GetGameInstance`)))
    (bind ((`OwningID_7_B372075A4A13A2336D81F6857A069E34` _owningid) (`SleeperGUID_16_625A7DD04788A2F9AC701AA1341AE7EF` _sleeperguid)) (break `/Game/n00dSleeper/Core/FN00dSleeper_Data` _sleepdata))
    (bind _structout_2 (setmembers `/Game/n00dSleeper/Core/FN00dSleeper_Data` :`StructRef` (`self.LoadedSleepData`) :`OwningID` _owningid :`SleeperGUID` _sleeperguid))
    (`self.ServerSetSleeperData` _structout_2)
    ;[1 1 1] Fade the vision
    (`self.SleepVisionStart`)
    (return)))

(fn `NotifyDeadSleeperPlayer`
  (params (Controller :type "Controller Object Reference"))
  (if (== Controller (`self.OwningController`))
    ;[0.2462 0.323 0.34] DEBUG
    (`self.Debug` "YOU DIED" "NewEnumerator4" "" false true 10.0)
    (return)
    (else
      (return))))

(fn `SetSleepData`
  (params (SleepData :type "/Game/n00dSleeper/Core/FN00dSleeper_Data Structure"))
  ;[1 1 1] Route us via the server if  we're the remote
  (`self.ControllerHasAuthority`
    (:`Authority`
      (set `self.LoadedSleepData` SleepData)
      ;[0.2462 0.323 0.34] DEBUG
      (`self.Debug` "Set LOADED SleepData for Player ID:" "NewEnumerator2" (`.OwningID_7_B372075A4A13A2336D81F6857A069E34` (break `/Game/n00dSleeper/Core/FN00dSleeper_Data` (`self.LoadedSleepData`))) false true 5.0)
      (return))
    (:`Remote`
      (return))))

(fn `SleeperSessionConnect`
  (params (IP_port :type String))
  ;[1 1 1] Connect to the session on the defined IP and Port
  (`KismetSystemLibrary.ExecuteConsoleCommand` (`KismetStringLibrary.Concat_StrStr` "open " IP_port) (`self.OwningPlayerController`))
  (return))

(fn `SleeperSessionOpen`
  ;[1 1 1] Open the test map as a listen server
  (`KismetSystemLibrary.ExecuteConsoleCommand` (`KismetStringLibrary.Concat_StrStr` "open " (`self.DebugMapName`) "?listen") (`self.OwningPlayerController`))
  (return))

(fn `SleepVisionStart`
  ;[1 1 1] Set the camera manager's camera fade function and a custom timer informing when to start fade. This will happen on the local controller
  (if (`self.UseScreenFade`)
    (`PlayerCameraManager.SetManualCameraFade` :`self` (`PlayerController.PlayerCameraManager` (`GameplayStatics.GetPlayerController` 0)) :`InFadeAmount` 1.0)
    (bind _returnvalue (`KismetSystemLibrary.K2_SetTimer` null "SleepVisionTimer" (`self.SleepVisionFadeDelay`)))
    (set `self.SleepVision` _returnvalue)
    (return)
    (else
      (return))))

(fn `SleepVisionTimer`
  ;[1 1 1] This will always be fired from the remote, so we can use get player controller here
  (`PlayerCameraManager.StartCameraFade` :`self` (`PlayerController.PlayerCameraManager` (`GameplayStatics.GetPlayerController` 0)) :`FromAlpha` 1.0 :`Duration` (- (`AnimSequenceBase.SequenceLength` (`.FromSleep_6_BE4A8AAA4058BC40F7E3B995B7FC0BD9` (break `/Game/n00dSleeper/Core/FN00dSleeper_Animation` (`.Animations_23_0C71528045C90A61DD4D64B48A4F1F75` (break `/Game/n00dSleeper/Core/FN00dSleeper_Data` (`self.LoadedSleepData`)))))) (`self.SleepVisionFadeDelay`)))
  (return))