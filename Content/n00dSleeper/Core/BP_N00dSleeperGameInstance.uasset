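; Game instance for the n00dSleeper system that owns sleeper save games and the local player's sleeper identity.
; On Init it loads or creates a server save on dedicated servers, or a client save otherwise.
; Non-dedicated instances then cache saved sleep data, generating and saving placeholder GUID-based IDs, meant to be swapped for a subsystem ID, when none are valid.
; Interface events and getters expose saving and data without casts.
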(event `self.ReceiveInit`
  ;[1 1 1] INTEGRATE ME
  ;;[0.09035 0.695 0.1803] Initialise
  (`self.LoadSleeperObject`)
  (`self.LoadSleeperData`))

(event `/Game/n00dSleeper/Core/BPI_N00dSleeper.SaveServerSleeperSlot`
  ;[1 1 1] INTEGRATE ME
  ;;[1 1 1] Interface Events
  (`GameplayStatics.SaveGameToSlot` (`self.ServerSleeperSave`) (`self.ServerSaveSlot`)))

(event `SaveSleeperObject`
  ;[1 1 1] INTEGRATE ME
  ;;[1 0.9455 0.1593] Serialisation
  ;;;[1 1 1] Save Sleeper Object
  (if (`KismetSystemLibrary.IsDedicatedServer`)
    (bind _returnvalue (`GameplayStatics.SaveGameToSlot` (`self.ServerSleeperSave`) (`self.ServerSaveSlot`)))
    (if _returnvalue
      (`KismetSystemLibrary.PrintString` "Server SUCCEEDED in Saving Game to Slot" true true (struct :`R` 0.09035 :`G` 0.695 :`B` 0.180317 :`A` 1.0) 2.0)
      (else
        (`KismetSystemLibrary.PrintString` "Server FAILED to Save Game to Slot" true true (struct :`R` 1.0 :`G` 0.05 :`B` 0.05 :`A` 1.0) 10.0)))
    (else
      (bind _returnvalue_2 (`GameplayStatics.SaveGameToSlot` (`self.ClientSleeperSave`) (`self.ClientSaveSlot`)))
      (if _returnvalue_2
        (`KismetSystemLibrary.PrintString` "SUCCEEDED in Saving Game to Slot" true true (struct :`R` 0.09035 :`G` 0.695 :`B` 0.180317 :`A` 1.0) 2.0)
        (else
          (`KismetSystemLibrary.PrintString` "FAILED to Save Game to Slot" true true (struct :`R` 1.0 :`G` 0.05 :`B` 0.05 :`A` 1.0) 10.0))))))

(event `LoadSleeperObject`
  (bind _serversaveslot (`self.ServerSaveSlot`))
  (bind _clientsaveslot (`self.ClientSaveSlot`))
  ;[1 1 1] INTEGRATE ME
  ;;[1 0.9455 0.1593] Serialisation
  ;;;[1 1 1] Load Sleeper Object
  (if (`KismetSystemLibrary.IsDedicatedServer`) :!label _label
    (`/Engine/EditorBlueprintResources/StandardMacros.IsValid` (`self.ServerSleeperSave`)
      (:`Is Valid`
        _)
      (:`Is Not Valid`
        (bind _returnvalue (`GameplayStatics.CreateSaveGameObject` "/Game/n00dSleeper/Core/BP_N00dSleeperSaveServer.BP_N00dSleeperSaveServer_C"))
        (set `self.ServerSleeperSave` _returnvalue)))
    (bind _returnvalue_2 (`GameplayStatics.DoesSaveGameExist` (`self.ServerSaveSlot`)))
    (if _returnvalue_2
      (bind _returnvalue_3 (`GameplayStatics.LoadGameFromSlot` _serversaveslot))
      (bind _asbp_n00d_sleeper_save_server (cast `/Game/n00dSleeper/Core/BP_N00dSleeperSaveServer` _returnvalue_3))
      (set `self.ServerSleeperSave` _asbp_n00d_sleeper_save_server)
      (`KismetSystemLibrary.PrintString` "SAVE LOADED on SERVER" true true (struct :`R` 0.09035 :`G` 0.695 :`B` 0.180317 :`A` 1.0))
      (else
        (bind _returnvalue_4 (`GameplayStatics.SaveGameToSlot` (`self.ServerSleeperSave`) _serversaveslot))
        (if _returnvalue_4
          (`KismetSystemLibrary.PrintString` "INITIAL SAVE on the SERVER" true true (struct :`R` 0.09035 :`G` 0.695 :`B` 0.180317 :`A` 1.0))
          (else
            (`KismetSystemLibrary.PrintString` "INITIAL SAVE on the SERVER FAILED" true true (struct :`R` 1.0 :`G` 0.05 :`B` 0.05 :`A` 1.0) 10.0)))))
    (else
      (`/Engine/EditorBlueprintResources/StandardMacros.IsValid` (`self.ClientSleeperSave`)
        (:`Is Valid`
          _)
        (:`Is Not Valid`
          (bind _returnvalue_5 (`GameplayStatics.CreateSaveGameObject` "/Game/n00dSleeper/Core/BP_N00dSleeperSaveClient.BP_N00dSleeperSaveClient_C"))
          (set `self.ClientSleeperSave` _returnvalue_5)))
      (bind _returnvalue_6 (`GameplayStatics.DoesSaveGameExist` (`self.ClientSaveSlot`)))
      (if _returnvalue_6
        (bind _returnvalue_7 (`GameplayStatics.LoadGameFromSlot` _clientsaveslot))
        (bind _asbp_n00d_sleeper_save_client (cast `/Game/n00dSleeper/Core/BP_N00dSleeperSaveClient` _returnvalue_7))
        (set `self.ClientSleeperSave` _asbp_n00d_sleeper_save_client)
        (`KismetSystemLibrary.PrintString` "SUCCEEDED in Loading Client Game from Slot" true true (struct :`R` 0.09035 :`G` 0.695 :`B` 0.180317 :`A` 1.0))
        (else
          (bind _returnvalue_8 (`GameplayStatics.SaveGameToSlot` (`self.ClientSleeperSave`) _clientsaveslot))
          (if _returnvalue_8
            (`KismetSystemLibrary.PrintString` "SUCCEEDED in Saving Client Game to Slot" true true (struct :`R` 0.09035 :`G` 0.695 :`B` 0.180317 :`A` 1.0))
            (else
              (`KismetSystemLibrary.PrintString` "FAILED to Save Client Game to Slot" true true (struct :`R` 1.0 :`G` 0.05 :`B` 0.05 :`A` 1.0) 10.0))))))))

(event `CreateListenServerSave`
  ;[1 1 1] INTEGRATE ME
  ;;[1 0.9455 0.1593] Serialisation
  ;;;[1 1 1] Load Sleeper Object
  (goto _label))

(event `LoadSleeperData`
  (bind _returnvalue (`KismetGuidLibrary.NewGuid`))
  (bind ((`OwningID_7_B372075A4A13A2336D81F6857A069E34` _owningid) (`SleeperGUID_16_625A7DD04788A2F9AC701AA1341AE7EF` _sleeperguid)) (break `/Game/n00dSleeper/Core/FN00dSleeper_Data` (`/Game/n00dSleeper/Core/BP_N00dSleeperSaveClient.SavedSleepData` (`self.ClientSleeperSave`))))
  ;[1 1 1] INTEGRATE ME
  ;;[1 0.9455 0.1593] Serialisation
  ;;;[1 1 1] Load Client Sleeper GUID from Save
  (if (not (`KismetSystemLibrary.IsDedicatedServer`))
    (if (and (`KismetStringLibrary.NotEqual_StrStr` _owningid "00000000000000000000000000000000") (`KismetStringLibrary.NotEqual_StrStr` _owningid))
      (set `self.LoadedSleepData` (`/Game/n00dSleeper/Core/BP_N00dSleeperSaveClient.SavedSleepData` (`self.ClientSleeperSave`)) :!label _label_2) ; Load the sleep data if the ID is valid
      (`KismetSystemLibrary.PrintString` "Sleep Data LOADED on the GameInstance" true true (struct :`R` 0.09035 :`G` 0.695 :`B` 0.180317 :`A` 1.0))
      (elif (`KismetGuidLibrary.IsValid_Guid` _sleeperguid)
        (goto _label_2)
        (else
          (bind _structout (setmembers `/Game/n00dSleeper/Core/FN00dSleeper_Data` :`StructRef` (`/Game/n00dSleeper/Core/BP_N00dSleeperSaveClient.SavedSleepData` (`self.ClientSleeperSave`)) :`OwningID` (`KismetGuidLibrary.Conv_GuidToString` _returnvalue) :`SleeperGUID` _returnvalue))
          (set `self.LoadedSleepData` _structout)
          (`self.SaveSleeperObject`)
          (`KismetSystemLibrary.PrintString` "Sleep Data SAVED on the GameInstance" true true (struct :`R` 0.09035 :`G` 0.695 :`B` 0.180317 :`A` 1.0)))))))

(fn `GetClientSleeperSave`
  (returns (ClientSave :type "/Game/n00dSleeper/Core/BP_N00dSleeperSaveClient Object Reference"))
  (return (`self.ClientSleeperSave`)))

(fn `GetControllerSleeper`
  (returns (ControllerSleeperComponent :type "/Game/n00dSleeper/Core/BPC_N00dSleeper_Controller Object Reference"))
  (return null))

(fn `GetGameModeSleeper`
  (returns (GameModeSleepComponent :type "/Game/n00dSleeper/Core/BPC_N00dSleeper_GameMode Object Reference"))
  (return null))

(fn `GetServerSleeperSave`
  (returns (ServerSave :type "/Game/n00dSleeper/Core/BP_N00dSleeperSaveServer Object Reference"))
  (return (`self.ServerSleeperSave`)))

(fn `GetSleepData`
  (returns (SleepData :type "/Game/n00dSleeper/Core/FN00dSleeper_Data Structure"))
  ;[1 1 1] Calling this avoids a cast in other BPs
  (return (`self.LoadedSleepData`)))