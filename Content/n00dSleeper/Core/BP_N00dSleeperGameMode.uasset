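; Game mode for the n00dSleeper system, which handles player sleeper actors across login and logout.
; It forwards BeginPlay, logout and delayed post-login events to a BPCN00dSleeperGameMode component, which it exposes through GetGameModeSleeper.
; ChoosePlayerStart spawns players at their sleeper actor when valid, otherwise using the component's overridable fallback.
; EndPlay saves server sleeper data only when play ends in the editor.
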(event `self.ReceiveBeginPlay`
  (bind _bpc_n00dsleeper_gamemode (`self.BPC_N00dSleeper_GameMode`))
  ;[1 1 1] INTEGRATE ME
  ;;[1 1 1] Initialise
  (`parent.ReceiveBeginPlay`)
  (`/Game/n00dSleeper/Deprecated/N00dMasterComponent.Initialise` _bpc_n00dsleeper_gamemode (`/Game/n00dSleeper/Deprecated/N00dMasterComponent.Owning` _bpc_n00dsleeper_gamemode)))

(event `self.K2_PostLogin`
  (params (NewPlayer :type "PlayerController Object Reference"))
  ;[1 1 1] INTEGRATE ME
  ;;[1 1 1] Handle sleeper entry and exit
  (`parent.K2_PostLogin` NewPlayer)
  (`KismetSystemLibrary.Delay` 1.0) ; Short delay for client to be spawned . This cannot be avoided in BP
  (`/Game/n00dSleeper/Core/BPC_N00dSleeper_GameMode.OnSleeperPostLogin` (`self.BPC_N00dSleeper_GameMode`) NewPlayer))

(event `self.K2_OnLogout`
  (params (ExitingController :type "Controller Object Reference"))
  ;[1 1 1] INTEGRATE ME
  ;;[1 1 1] Handle sleeper entry and exit
  (`parent.K2_OnLogout` ExitingController)
  (`/Game/n00dSleeper/Core/BPC_N00dSleeper_GameMode.OnSleeperLogout` (`self.BPC_N00dSleeper_GameMode`) ExitingController))

(event `self.ReceiveEndPlay`
  (params (EndPlayReason :type "EEndPlayReason Enum" :default "Destroyed"))
  (switch `EEndPlayReason` EndPlayReason
    (:`EndPlayInEditor`
      (`/Game/n00dSleeper/Core/BPC_N00dSleeper_GameMode.SaveServerSleeperData` (`self.BPC_N00dSleeper_GameMode`)))))

(fn `ChoosePlayerStart`
  (params (Player :type "Controller Object Reference"))
  (returns (ReturnValue :type "Actor Object Reference"))
  (locals (LocalController :type "Controller Object Reference"))
  (bind _sleeperactor (`/Game/n00dSleeper/Core/BPC_N00dSleeper_GameMode.ChooseSleeperStart` (`self.BPC_N00dSleeper_GameMode`) (`local.LocalController`)))
  ;[1 1 1] Override to get our desired player start (owner's sleeper actor)
  (set `local.LocalController` Player)
  (`/Engine/EditorBlueprintResources/StandardMacros.IsValid` _sleeperactor
    (:`Is Valid`
      (return _sleeperactor) ; Return the sleeper actor
    )
    (:`Is Not Valid`
      ;;[1 1 1] Send the default spawning method to an overridable function
      (bind _playerstart (`/Game/n00dSleeper/Core/BPC_N00dSleeper_GameMode.CustomChoosePlayerStart` (`self.BPC_N00dSleeper_GameMode`)))
      (return _playerstart))))

(fn `GetClientSleeperSave`
  (returns (ClientSave :type "/Game/n00dSleeper/Core/BP_N00dSleeperSaveClient Object Reference"))
  (return null))

(fn `GetControllerSleeper`
  (returns (ControllerSleeperComponent :type "/Game/n00dSleeper/Core/BPC_N00dSleeper_Controller Object Reference"))
  (return null))

(fn `GetGameModeSleeper`
  (returns (GameModeSleepComponent :type "/Game/n00dSleeper/Core/BPC_N00dSleeper_GameMode Object Reference"))
  (return (`self.BPC_N00dSleeper_GameMode`)))

(fn `GetServerSleeperSave`
  (returns (ServerSave :type "/Game/n00dSleeper/Core/BP_N00dSleeperSaveServer Object Reference"))
  (return null))

(fn `GetSleepData`
  (returns (SleepData :type "/Game/n00dSleeper/Core/FN00dSleeper_Data Structure"))
  (return))

(fn `UserConstructionScript`
  (`parent.UserConstructionScript`))