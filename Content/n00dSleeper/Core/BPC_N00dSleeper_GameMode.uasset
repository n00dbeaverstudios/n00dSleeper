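; Game Mode component for n00dSleeper, leaving a sleeper actor in the world when a player logs out.
; On initialise it loads server sleep data through the Game Instance and respawns sleepers at their saved indices.
; Logout spawns and registers a sleeper; login finds it by OwningID and calls WakeUp.
; Killed sleepers are removed from world and save, and kept in an unsaved list that login checks to report death.
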(event `DeleteServerSave`
  ;[1 0.05 0.05] Delete the sleeper saves for client and server
  (`self.DeleteSave`))

(event `self.Initialise`
  (params (Owning :type "/Game/n00dSleeper/Deprecated/FOwning Structure"))
  ;[1 1 1] Initialise
  (`parent.Initialise` Owning)
  (`self.InitialiseGameMode`))

(fn `AddPlayerToSleeperArray`
  (params (ForController :type "Controller Object Reference"))
  (locals (LocalController :type "Controller Object Reference") (LocalSleepData :type "/Game/n00dSleeper/Core/FN00dSleeper_Data Structure"))
  (bind (_location _yaw) (`self.ResolveSleeperPostition` (`local.LocalController`)))
  ;[1 1 1] Get the player's sleep data and add it to the server array
  ;;[1 1 1] Cache and get data
  (bind _output_get (set `local.LocalController` ForController))
  (bind _sleepdata (message `/Game/n00dSleeper/Core/BPI_N00dSleeper.GetSleepData` _output_get))
  (set `local.LocalSleepData` _sleepdata)
  ;;[1 1 1] Add the sleep data to loaded server data
  (bind _returnvalue (`KismetArrayLibrary.Array_Add` (`self.LoadedServerSleepData`) (`local.LocalSleepData`)))
  ;;[1 1 1] Save the controller's position in the world in the player's server sleep data
  (setmembers `/Game/n00dSleeper/Core/FN00dSleeper_Data` :`StructRef` (`|GetArrayItem` (`self.LoadedServerSleepData`) _returnvalue) :`Location` _location :`Rotation` (`KismetMathLibrary.MakeRotator` 0.0 0.0 _yaw)) ; Set its members
  (`self.SaveServerSleeperData`)
  ;;[0.2462 0.323 0.34] DEBUG
  (`self.Debug` "ADDED PLAYER SLEEP DATA TO SERVER ARRAY" "NewEnumerator4")
  (return))

(fn `AddToActiveSleeperActors`
  (params (SleeperActor :type "/Game/n00dSleeper/Core/BP_N00dSleeperActor Object Reference") (ForController :type "Controller Object Reference") (SleepDataIndex :type Integer) (SleepActorIndex :type Integer))
  (locals (LocalSleeperActor :type "/Game/n00dSleeper/Core/BP_N00dSleeperActor Object Reference") (LocalController :type "Controller Object Reference") (LocalDataIndex :type Integer) (LocalActorIndex :type Integer) (LocalAdd :type Integer))
  (bind _loadedserversleepdata (`self.LoadedServerSleepData`))
  ;[1 1 1] Load the sleeper actors, or save the controller sleep actor and set its index in the loaded sleeper data
  ;;[1 1 1] Cache
  (set `local.LocalSleeperActor` SleeperActor)
  (set `local.LocalController` ForController)
  (set `local.LocalDataIndex` SleepDataIndex)
  (set `local.LocalActorIndex` SleepActorIndex)
  (`/Engine/EditorBlueprintResources/StandardMacros.IsValid` (`local.LocalController`) ; Have we got an incoming controller
    (:`Is Valid`
      ;;[1 1 1] If there is an active controller, lets save its sleep actor index on the server data for this controller. It means we're logging out (sleeping)
      ;;;[1 1 1] Add to active actors
      (bind _returnvalue (`KismetArrayLibrary.Array_Add` (`self.ActiveSleepActors`) (`local.LocalSleeperActor`)))
      (set `local.LocalAdd` _returnvalue)
      ;;;[1 1 1] Find the exiting controller's sleep data in the server save
      (bind _sleepdata (message `/Game/n00dSleeper/Core/BPI_N00dSleeper.GetSleepData` (`local.LocalController`))) ; Grab the sleep data from the controller
      (bind _returnvalue_2 (`KismetArrayLibrary.Array_Find` _loadedserversleepdata _sleepdata))
      (if (`KismetArrayLibrary.Array_IsValidIndex` _loadedserversleepdata _returnvalue_2)
        ;;;[1 1 1] Set the sleep actor index in the member of the server sleep data
        (setmembers `/Game/n00dSleeper/Core/FN00dSleeper_Data` :`StructRef` (`|GetArrayItem` _loadedserversleepdata _returnvalue_2) :`SleepActorIndex` (`local.LocalAdd`))
        ;;;[1 1 1] Save the changes
        (`self.SaveServerSleeperData`)
        (return)
        (else
          (return))))
    (:`Is Not Valid`
      ;;[1 1 1] If the controller is not valid that means we're loading the server, so set the sleep actor index from the save and reference the actor in the active list - this willl be looping
      ;;;[1 1 1] ...and map the actor index to the sleep data index the same as it was when saved
      (setmembers `/Game/n00dSleeper/Core/FN00dSleeper_Data` :`StructRef` (`|GetArrayItem` (`self.LoadedServerSleepData`) (`local.LocalDataIndex`)) :`SleepActorIndex` (`local.LocalActorIndex`))
      ;;;[1 1 1] Set array on the specified index (create array the same as it was)
      (`KismetArrayLibrary.Array_Set` (`self.ActiveSleepActors`) (`local.LocalActorIndex`) (`local.LocalSleeperActor`) true)
      (return))))

(fn `ChooseSleeperStart`
  (params (ForController :type "Controller Object Reference"))
  (returns (SleeperActor :type "/Game/n00dSleeper/Core/BP_N00dSleeperActor Object Reference"))
  (return (`|GetArrayItem` (`self.ActiveSleepActors`) (`.SleepActorIndex_20_43AFEB9740D88D28FA4A2D80BC7285DA` (break `/Game/n00dSleeper/Core/FN00dSleeper_Data` (`.ServerSleepData` (`self.GetServerSleepData` ForController)))))))

(fn `CustomChoosePlayerStart`
  (returns (PlayerStart :type "PlayerStart Object Reference"))
  ;[1 1 1] Override me to control how the player is spawned if no sleeper actor found for controller
  ;;[1 1 1] Loop the player starts and return the first one if there was no sleeper actor found for this controller. Swap this out for smarter ways to handle initial entry
  (bind _outactors (`GameplayStatics.GetAllActorsOfClass` "/Script/Engine.PlayerStart"))
  (for _array_element _outactors
    (return _array_element)))

(fn `DeleteSave`
  ;[1 1 1] Delete the sleep data on slot
  (bind _returnvalue (`GameplayStatics.DeleteGameInSlot` "SleeperSaveServer"))
  (if _returnvalue
    (`self.Debug` "DELETED Server Save" "NewEnumerator4")
    (else
      (`self.Debug` "NOTHING TO DELETE On Server" "NewEnumerator4")))
  (return))

(fn `GetServerSleepData`
  (params (ForController :type "Controller Object Reference"))
  (returns (Found :type Boolean) (ServerSleepData :type "/Game/n00dSleeper/Core/FN00dSleeper_Data Structure"))
  (locals (LocalController :type "Controller Object Reference") (LocalServer :type "/Game/n00dSleeper/Core/FN00dSleeper_Data Structure") (FoundData :type Boolean) (LocalControllerSD :type "/Game/n00dSleeper/Core/FN00dSleeper_Data Structure"))
  ;[1 1 1] Return the sleeper data for the matching ID
  ;;[1 1 1] Cache
  (bind _sleepdata (message `/Game/n00dSleeper/Core/BPI_N00dSleeper.GetSleepData` ForController))
  (set `local.LocalControllerSD` _sleepdata)
  ;;[1 1 1] Loop the active sleepers and continue when we've found a server save that matches the controller's
  (for _array_element (`self.ActiveSleepActors`)
    (bind _sleepdata_2 (`/Game/n00dSleeper/Core/BP_N00dSleeperActor.SleepData` _array_element))
    (if (`KismetStringLibrary.EqualEqual_StrStr` (`.OwningID_7_B372075A4A13A2336D81F6857A069E34` (break `/Game/n00dSleeper/Core/FN00dSleeper_Data` _sleepdata_2)) (`.OwningID_7_B372075A4A13A2336D81F6857A069E34` (break `/Game/n00dSleeper/Core/FN00dSleeper_Data` (`local.LocalControllerSD`))))
      (set `local.LocalServer` _sleepdata_2)
      (set `local.FoundData` true)))
  (return (`local.FoundData`) (`local.LocalServer`)))

(fn `GetSleepActor`
  (params (ForController :type "Controller Object Reference"))
  (returns (SleepActor :type "/Game/n00dSleeper/Core/BP_N00dSleeperActor Object Reference"))
  (return (`|GetArrayItem` (`self.ActiveSleepActors`) (`.SleepActorIndex_20_43AFEB9740D88D28FA4A2D80BC7285DA` (break `/Game/n00dSleeper/Core/FN00dSleeper_Data` (`.ServerSleepData` (`self.GetServerSleepData` ForController)))))))

(fn `InitialiseGameMode`
  ;[0.09035 0.695 0.1803] Initialise Game Mode Sleeper Component
  ;;[1 1 1] Store a reference to the owner
  (set `self.OwningGameMode` (cast `GameMode` (`self.GetOwner`) :!pure true))
  ;;[1 1 1] LOAD
  ;;;[1 1 1] Load the server save game object
  (`self.LoadServerFromSlot`)
  ;;;[1 1 1] Load the array from the save to an active reference
  (`self.LoadServerSleeperData`)
  ;;;[1 1 1] Load a sleep actor for each sleep data found in the array
  (`self.LoadServerSleeperActors`)
  (return))

(fn `IsSleeperDead`
  (params (ForController :type "Controller Object Reference"))
  (returns (Dead :type Boolean))
  (locals (FoundData :type Boolean) (LocalServer :type "/Game/n00dSleeper/Core/FN00dSleeper_Data Structure") (LocalControllerSD :type "/Game/n00dSleeper/Core/FN00dSleeper_Data Structure"))
  ;[1 1 1] Cache
  (bind _sleepdata (message `/Game/n00dSleeper/Core/BPI_N00dSleeper.GetSleepData` ForController))
  (set `local.LocalControllerSD` _sleepdata)
  ;[1 1 1] See if this controller is on the dead sleepers list
  (for _array_element (`self.DeadSleepers`)
    (if (`KismetStringLibrary.EqualEqual_StrStr` (`.OwningID_7_B372075A4A13A2336D81F6857A069E34` (break `/Game/n00dSleeper/Core/FN00dSleeper_Data` _array_element)) (`.OwningID_7_B372075A4A13A2336D81F6857A069E34` (break `/Game/n00dSleeper/Core/FN00dSleeper_Data` (`local.LocalControllerSD`))))
      (set `local.FoundData` true)))
  (return (`local.FoundData`)))

(fn `KillSleeper`
  (params (SleepData :type "/Game/n00dSleeper/Core/FN00dSleeper_Data Structure"))
  (locals (LocalDeadSleeper :type "/Game/n00dSleeper/Core/FN00dSleeper_Data Structure") (FoundData :type Boolean) (LocalServerPlayer :type "/Game/n00dSleeper/Core/FN00dSleeper_Data Structure") (LocalSleepActor :type "/Game/n00dSleeper/Core/BP_N00dSleeperActor Object Reference"))
  ;[1 1 1] Cache dead player
  (bind _output_get (set `local.LocalDeadSleeper` SleepData))
  (`KismetArrayLibrary.Array_Add` (`self.DeadSleepers`) _output_get)
  ;[1 1 1] Loop the active sleeper actors and remove the player from the server when we've found a save that matches the dead sleeper
  (for _array_element (`self.ActiveSleepActors`)
    (bind _sleepdata (`/Game/n00dSleeper/Core/BP_N00dSleeperActor.SleepData` _array_element))
    (if (`KismetStringLibrary.EqualEqual_StrStr` (`.OwningID_7_B372075A4A13A2336D81F6857A069E34` (break `/Game/n00dSleeper/Core/FN00dSleeper_Data` _sleepdata)) (`.OwningID_7_B372075A4A13A2336D81F6857A069E34` (break `/Game/n00dSleeper/Core/FN00dSleeper_Data` (`local.LocalDeadSleeper`))))
      (set `local.LocalServerPlayer` _sleepdata)
      (set `local.FoundData` true)
      (set `local.LocalSleepActor` _array_element)))
  (if (`local.FoundData`)
    (`KismetArrayLibrary.Array_RemoveItem` (`self.LoadedServerSleepData`) (`local.LocalServerPlayer`))
    (`self.SaveServerSleeperData`)
    (`self.RemoveSleepActor` (`local.LocalSleepActor`))
    ;;[0.2462 0.323 0.34] DEBUG
    (`self.Debug` (`KismetStringLibrary.Concat_StrStr` (`.OwningID_7_B372075A4A13A2336D81F6857A069E34` (break `/Game/n00dSleeper/Core/FN00dSleeper_Data` (`local.LocalServerPlayer`))) " is DEAD") "NewEnumerator4" "" false true 10.0)
    (return)
    (else
      (return))))

(fn `LoadServerFromSlot`
  ;[1 1 1] Store a reference to the save object from the server game instance
  (bind _serversave (message `/Game/n00dSleeper/Core/BPI_N00dSleeper.GetServerSleeperSave` (`GameplayStatics.GetGameInstance`)))
  (set `self.ServerSave` _serversave)
  (return))

(fn `LoadServerSleeperActors`
  (locals (LocalElement :type Integer) (LocalCount :type Integer))
  ;[1 1 1] Spawn a sleeper actor for each sleep data found on the server
  ;;[1 1 1] Loops the loaded sleep data and grab its location and index
  (for (_array_element _array_index) (`self.LoadedServerSleepData`)
    (set `local.LocalElement` _array_index)
    (bind ((`SleepActorIndex_20_43AFEB9740D88D28FA4A2D80BC7285DA` _sleepactorindex) (`Location_26_A8C917AB4127A8BA4FB850BA4A5C61D7` _location) (`Rotation_29_9C493C3448359FCDCE17268620ACF414` _rotation)) (break `/Game/n00dSleeper/Core/FN00dSleeper_Data` _array_element))
    ;;[1 1 1] Spawn the Sleeper Actor per element at the loaded location and rotation
    (bind _returnvalue (`|SpawnActorFromClass` "/Game/n00dSleeper/Core/BP_N00dSleeperActor.BP_N00dSleeperActor_C" (`KismetMathLibrary.MakeTransform` _location _rotation) "Undefined" "OverrideRootScale" null _array_element))
    ;;[1 1 1] Save these
    (`self.AddToActiveSleeperActors` _returnvalue null (`local.LocalElement`) _sleepactorindex)
    ;;[1 1 1] Increment local Int
    (`/Engine/EditorBlueprintResources/StandardMacros.IncrementInt` (`local.LocalCount`)))
  ;;[0.2462 0.323 0.34] DEBUG
  (`self.Debug` (`KismetStringLibrary.Concat_StrStr` (`KismetStringLibrary.Conv_IntToString` (`local.LocalCount`)) " Sleep Actor(s) Loaded on Server") "NewEnumerator4" "" false true 10.0))

(fn `LoadServerSleeperData`
  (bind _serversave (`self.ServerSave`))
  ;[1 1 1] Load the data from the save object
  (`/Engine/EditorBlueprintResources/StandardMacros.IsValid` _serversave
    (:`Is Valid`
      (set `self.LoadedServerSleepData` (`/Game/n00dSleeper/Core/BP_N00dSleeperSaveServer.SleepData` _serversave)))
    (:`Is Not Valid`
      _))
  (return))

(fn `OnSleeperLogout`
  (params (ForController :type "Controller Object Reference"))
  (locals (LocalExiting :type "Controller Object Reference") (LocalServerSleepData :type "/Game/n00dSleeper/Core/FN00dSleeper_Data Structure"))
  (bind _localexiting (`local.LocalExiting`))
  ;[1 1 1] Spawn the sleep actor for the controller, save it to the server, and set the actor's sleep data
  ;;[1 1 1] Add the exiting controller to the server save array
  (set `local.LocalExiting` ForController)
  ;;[1 1 1] Check if the server has a save for this controller
  (if (not (`self.GetServerSleepData` (`local.LocalExiting`)))
    ;;[1 1 1] And add the existing controller sleep data to the sleep array
    (`self.AddPlayerToSleeperArray` (`local.LocalExiting`)))
  ;;[1 1 1] Spawn the sleeper actor in the world at the player's location and with the controller's sleep data
  (bind _sleepactor (`self.SpawnSleepActor` (`local.LocalExiting`)))
  (`/Engine/EditorBlueprintResources/StandardMacros.IsValid` _sleepactor
    (:`Is Valid`
      ;;[1 1 1] Send the controller's sleep data to the sleeper actor
      (bind _sleepdata (message `/Game/n00dSleeper/Core/BPI_N00dSleeper.GetSleepData` _localexiting))
      (`/Game/n00dSleeper/Core/BP_N00dSleeperActor.FallAsleep` _sleepactor _sleepdata _localexiting)
      ;;[0.2462 0.323 0.34] DEBUG
      (`self.Debug` "Spawned Sleep Actor:" "NewEnumerator2" (`KismetSystemLibrary.GetDisplayName` _sleepactor))
      (return))
    (:`Is Not Valid`
      ;;[0.2462 0.323 0.34] DEBUG
      (`self.Debug` "SLEEPER ACTOR Not Valid" "NewEnumerator4" "" false false 20.0)
      (return))))

(fn `OnSleeperPostLogin`
  (params (ForController :type "Controller Object Reference"))
  (locals (LocalServerSleepData :type "/Game/n00dSleeper/Core/FN00dSleeper_Data Structure") (LocalController :type "Controller Object Reference"))
  (bind (_found _serversleepdata) (`self.GetServerSleepData` (`local.LocalController`)))
  (bind _sleeperactor (`self.ChooseSleeperStart` (`local.LocalController`)))
  ;[1 1 1] Handle player login
  ;;[1 1 1] Cache
  (set `local.LocalController` ForController)
  ;;[1 1 1] See if this controller's SleepData exists on the server
  (if _found
    ;;[0.2462 0.323 0.34] DEBUG
    ;;;[1 1 1] Set the sleeper data from server on the controller for debug and client server comparison
    (message `/Game/n00dSleeper/Core/BPI_N00dSleeper.SetDebugSleepData` (`local.LocalController`) _serversleepdata) ; Set the debug sleep data on the controller
    ;;[1 1 1] Get the sleeper actor and send a wake up call on the owner's sleep actor
    (`/Engine/EditorBlueprintResources/StandardMacros.IsValid` _sleeperactor
      (:`Is Valid`
        (`/Game/n00dSleeper/Core/BP_N00dSleeperActor.WakeUp` _sleeperactor (`local.LocalController`))
        (return))
      (:`Is Not Valid`
        ;;[0.2462 0.323 0.34] DEBUG
        (`self.Debug` "SLEEPER ACTOR Not Valid" "NewEnumerator4" "" false false 20.0)
        (return)))
    (else
      ;;[1 1 1] Check that we aren't dead
      (if (`self.IsSleeperDead` (`local.LocalController`))
        ;;[1 1 1] Send the confirmation off to a delegate on the controller
        (`self.OnSleeperDead` (`local.LocalController`))
        (return)
        (else
          ;;[0.2462 0.323 0.34] DEBUG
          (`self.Debug` "SERVER SAVE for CONTROLLER NOT FOUND - Is this your first log in attempt, or have you defined the correct Game Instance in the Project Settings" "NewEnumerator4" "" false false 20.0)
          (return))))))

(fn `RemovePlayerFromLoadedSleepData`
  (params (ForController :type "Controller Object Reference"))
  (bind (_found _serversleepdata) (`self.GetServerSleepData` ForController))
  ;[1 1 1] Find the player on the server, and remove the sleeper data from the array
  (if _found
    (`KismetArrayLibrary.Array_RemoveItem` (`self.LoadedServerSleepData`) _serversleepdata)
    (`self.SaveServerSleeperData`)
    (return)
    (else
      (return))))

(fn `RemoveSleepActor`
  (params (SleepActorToRemove :type "/Game/n00dSleeper/Core/BP_N00dSleeperActor Object Reference"))
  (locals (LocalSleepActor :type "/Game/n00dSleeper/Core/BP_N00dSleeperActor Object Reference"))
  (bind _localsleepactor (`local.LocalSleepActor`))
  ;[1 1 1] Handle the sleeper actor
  ;;[1 1 1] Cache
  (set `local.LocalSleepActor` SleepActorToRemove)
  ;;[0.2462 0.323 0.34] DEBUG
  (`self.Debug` (`KismetStringLibrary.Concat_StrStr` "REMOVED SLEEP ACTOR: " (`KismetSystemLibrary.GetDisplayName` _localsleepactor) " on INDEX: " (`KismetStringLibrary.Conv_IntToString` (`KismetArrayLibrary.Array_Find` (`self.ActiveSleepActors`) _localsleepactor))) "NewEnumerator4" "" false true 5.0)
  ;;[1 1 1] Remove the incoming from the array
  (`KismetArrayLibrary.Array_RemoveItem` (`self.ActiveSleepActors`) (`local.LocalSleepActor`))
  ;;[1 1 1] Destroy it and return
  (`Actor.K2_DestroyActor` (`local.LocalSleepActor`))
  (return))

(fn `ResolveSleeperPostition`
  (params (SleeperActor :type "Actor Object Reference"))
  (returns (Location :type "Vector Structure") (Yaw :type "Float (double-precision)"))
  (bind (_returnvalue_roll _returnvalue_pitch _returnvalue_yaw) (`KismetMathLibrary.BreakRotator` (`Actor.K2_GetActorRotation` SleeperActor)))
  ;[1 1 1] Set the sleeper actor as the incoming location and rotation
  (return (`Actor.K2_GetActorLocation` SleeperActor) _returnvalue_yaw))

(fn `SaveServerSleeperData`
  (bind _returnvalue (`GameplayStatics.GetGameInstance`))
  ;[1 1 1] Send messages to the game instance to set and save the server data
  (message `/Game/n00dSleeper/Core/BPI_N00dSleeper.SetServerSleepData` _returnvalue (`self.LoadedServerSleepData`))
  (message `/Game/n00dSleeper/Core/BPI_N00dSleeper.SaveServerSleeperSlot` _returnvalue)
  (return))

(fn `SpawnSleepActor`
  (params (ForController :type "Controller Object Reference"))
  (returns (SleepActor :type "/Game/n00dSleeper/Core/BP_N00dSleeperActor Object Reference"))
  (locals (LocalController :type "Controller Object Reference") (LocalSleepActor :type "/Game/n00dSleeper/Core/BP_N00dSleeperActor Object Reference"))
  (bind _localcontroller (`local.LocalController`))
  (bind (_location _yaw) (`self.ResolveSleeperPostition` (`local.LocalController`)))
  ;[1 1 1] Spawn the sleep actor and set the owner SleepData in the recently spawned actor - add them to an array to call on later, such as logon
  (bind _output_get (set `local.LocalController` ForController))
  (bind _sleepdata (message `/Game/n00dSleeper/Core/BPI_N00dSleeper.GetSleepData` _output_get))
  (bind _returnvalue (`|SpawnActorFromClass` (`self.SleeperActorClass`) (`KismetMathLibrary.MakeTransform` _location (`KismetMathLibrary.MakeRotator` 0.0 0.0 _yaw)) "AdjustIfPossibleButAlwaysSpawn" "OverrideRootScale" _localcontroller _sleepdata _localcontroller (`Actor.Instigator` _localcontroller)))
  ;;[0.2462 0.323 0.34] DEBUG
  (`self.Debug` "SLEEP ACTOR LOCATION: " "NewEnumerator2" (`KismetStringLibrary.Conv_VectorToString` _location) false true 10.0)
  ;;[1 1 1] Add the spawned sleep actor to an array
  (bind _output_get_2 (set `local.LocalSleepActor` _returnvalue))
  (`self.AddToActiveSleeperActors` _output_get_2 (`local.LocalController`))
  (return _output_get_2))