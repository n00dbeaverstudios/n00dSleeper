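; Player controller for the n00dSleeper system, acting as the owner and access point for its sleeper controller component.
; Construction sets component defaults, and BeginPlay passes the controller and possessed Character's mesh to the component.
; BPI_N00dSleeper getters expose the component and its loaded sleep data, while game mode and save getters are empty.
; Debug hooks open or join a listen server session on O/L and forward server-sent sleep data for comparison.
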(event `self.ReceiveBeginPlay`
  (`parent.ReceiveBeginPlay`)
  ;[1 1 1] COPY ME
  ;;[1 1 1] Initialise Sleeper for Controller
  (bind _ascharacter (cast `Character` (`self.K2_GetPawn`)))
  (bind _structout (setmembers `/Game/n00dComponents/Core/FOwning` :`StructRef` (`/Game/n00dComponents/Core/N00dMasterComponent.Owning` (`self.BPC_N00dSleeper_Controller`)) :`Controller` self :`PlayerController` self :`SkeletalMesh` (`Character.Mesh` _ascharacter)))
  (`/Game/n00dComponents/Core/N00dMasterComponent.Initialise` (`self.BPC_N00dSleeper_Controller`) _structout))

(event `Key|O`
  (params (Key :type "Key Structure" :default "AnyKey"))
  ;[1 1 1] COPY ME
  ;;[1 1 1] DEBUG - GameInstance needs to be applied in Migrate Project
  ;;;[1 1 1] Open a Listen server session (make sure to delete N00dDocs from map before building as it tries to call Billboard before its created)
  (:`Pressed`
    (`/Game/n00dComponents/n00dPacks/n00dGameplay/n00dSleeper/Blueprints/BPC_N00dSleeper_Controller.SleeperSessionOpen` (`self.BPC_N00dSleeper_Controller`))))

(event `Key|L`
  (params (Key :type "Key Structure" :default "AnyKey"))
  (bind _bpc_n00dsleeper_controller (`self.BPC_N00dSleeper_Controller`))
  ;[1 1 1] COPY ME
  ;;[1 1 1] DEBUG - GameInstance needs to be applied in Migrate Project
  ;;;[1 1 1] Open a local connection to a listen server
  (:`Pressed`
    (`/Game/n00dComponents/n00dPacks/n00dGameplay/n00dSleeper/Blueprints/BPC_N00dSleeper_Controller.SleeperSessionConnect` _bpc_n00dsleeper_controller (`/Game/n00dComponents/n00dPacks/n00dGameplay/n00dSleeper/Blueprints/BPC_N00dSleeper_Controller.InternalIP` _bpc_n00dsleeper_controller))))

(event `/Game/n00dComponents/n00dPacks/n00dGameplay/n00dSleeper/Blueprints/BPI_N00dSleeper.SetDebugSleepData`
  (params (SleepData :type "/Game/n00dComponents/n00dPacks/n00dGameplay/n00dSleeper/Blueprints/FN00dSleeper_Data Structure"))
  ;[1 1 1] COPY ME
  ;;[1 1 1] Sent from Game Mode as Server SleepData - for debug and security compare
  (`/Game/n00dComponents/n00dPacks/n00dGameplay/n00dSleeper/Blueprints/BPC_N00dSleeper_Controller.OwningSleepDataFromServer` (`self.BPC_N00dSleeper_Controller`) SleepData))

(fn `GetClientSleeperSave`
  (returns (ClientSave :type "/Game/n00dComponents/n00dPacks/n00dGameplay/n00dSleeper/Blueprints/BP_N00dSleeperSaveClient Object Reference"))
  (return null))

(fn `GetControllerSleeper`
  (returns (ControllerSleeperComponent :type "/Game/n00dComponents/n00dPacks/n00dGameplay/n00dSleeper/Blueprints/BPC_N00dSleeper_Controller Object Reference"))
  (return (`self.BPC_N00dSleeper_Controller`)))

(fn `GetGameModeSleeper`
  (returns (GameModeSleepComponent :type "/Game/n00dComponents/n00dPacks/n00dGameplay/n00dSleeper/Blueprints/BPC_N00dSleeper_GameMode Object Reference"))
  (return null))

(fn `GetServerSleeperSave`
  (returns (ServerSave :type "/Game/n00dComponents/n00dPacks/n00dGameplay/n00dSleeper/Blueprints/BP_N00dSleeperSaveServer Object Reference"))
  (return null))

(fn `GetSleepData`
  (returns (SleepData :type "/Game/n00dComponents/n00dPacks/n00dGameplay/n00dSleeper/Blueprints/FN00dSleeper_Data Structure"))
  ;[1 1 1] Parse the component's sleep data to BPI_N00dSleeper
  (return (`/Game/n00dComponents/n00dPacks/n00dGameplay/n00dSleeper/Blueprints/BPC_N00dSleeper_Controller.LoadedSleepData` (`self.BPC_N00dSleeper_Controller`))))

(fn `UserConstructionScript`
  ;[1 1 1] Set the component animations in the loaded sleep data
  (`parent.UserConstructionScript`)
  (`/Game/n00dComponents/n00dPacks/n00dGameplay/n00dSleeper/Blueprints/BPC_N00dSleeper_Controller.ConstuctDefaults` (`self.BPC_N00dSleeper_Controller`)))