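; Server-side save game for the n00dSleeper system that stores an array of player sleep data and writes itself to the server save slot.
; Functions replace the whole array, add missing entries, remove a player's entry or update its location and rotation, matching entries by SleeperGUID.
; Removal and location updates get the GUID from the controller's sleep data message.
; SaveServerSleeperActor is an empty stub.
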(fn `RemovePlayerSleepDataFromArray`
  (params (ForController :type "Controller Object Reference"))
  (locals (LocalSleepData :type "/Game/n00dComponents/n00dPacks/n00dGameplay/n00dSleeper/Blueprints/FN00dSleeper_Data Structure") (LocalSleeperForControllerGUID :type "Guid Structure") (LocalExisitingGUID :type Boolean) (LocalArrayElement :type Integer))
  (bind _sleepdata (`self.SleepData`))
  ;[1 1 1] Look for the incoming player in the server array and remove it if found
  ;;[1 1 1] Cache
  (bind _sleepdata_2 (message `/Game/n00dComponents/n00dPacks/n00dGameplay/n00dSleeper/Blueprints/BPI_N00dSleeper.GetSleepData` ForController))
  (set `local.LocalSleepData` _sleepdata_2)
  (set `local.LocalSleeperForControllerGUID` (`.SleeperGUID_16_625A7DD04788A2F9AC701AA1341AE7EF` (break `/Game/n00dComponents/n00dPacks/n00dGameplay/n00dSleeper/Blueprints/FN00dSleeper_Data` _sleepdata_2)))
  ;;[1 1 1] Look for the incoming GUID in the array and see if it matches the incoming. Mark it as existing if we find one
  (for (_array_element _array_index) (`self.SleepData`)
    (if (== (`local.LocalSleeperForControllerGUID`) (`.SleeperGUID_16_625A7DD04788A2F9AC701AA1341AE7EF` (break `/Game/n00dComponents/n00dPacks/n00dGameplay/n00dSleeper/Blueprints/FN00dSleeper_Data` _array_element)))
      (set `local.LocalExisitingGUID` true)
      (set `local.LocalArrayElement` _array_index)))
  ;;[1 1 1] Return if not found or remove player from array then save to disk
  (if (`local.LocalExisitingGUID`)
    (`KismetArrayLibrary.Array_RemoveItem` _sleepdata (`|GetArrayItem` _sleepdata (`local.LocalArrayElement`))) ; and remove this player from the array
    (`GameplayStatics.SaveGameToSlot` self (`self.ServerSaveSlot`)))
  (return))

(fn `SaveServerGameModeSleeperData`
  (params (SleepData :type "Array of /Game/n00dComponents/n00dPacks/n00dGameplay/n00dSleeper/Blueprints/FN00dSleeper_Data Structure"))
  (returns (Saved :type Boolean))
  (`|ExecutionSequence`
    (:`then_0`
      (set `self.SleepData` SleepData))
    (:`then_1`
      (bind _returnvalue (`GameplayStatics.SaveGameToSlot` self (`self.ServerSaveSlot`)))
      (return _returnvalue))))

(fn `SaveServerSleeperActor`)

(fn `SaveServerSleeperData`
  (params (SleepDataForController :type "/Game/n00dComponents/n00dPacks/n00dGameplay/n00dSleeper/Blueprints/FN00dSleeper_Data Structure"))
  (returns (Saved :type Boolean))
  (locals (LocalFound :type Boolean) (LocalSleepData :type "/Game/n00dComponents/n00dPacks/n00dGameplay/n00dSleeper/Blueprints/FN00dSleeper_Data Structure"))
  (for _array_element (`self.SleepData`)
    (if (== (`.SleeperGUID_16_625A7DD04788A2F9AC701AA1341AE7EF` (break `/Game/n00dComponents/n00dPacks/n00dGameplay/n00dSleeper/Blueprints/FN00dSleeper_Data` _array_element)) (`.SleeperGUID_16_625A7DD04788A2F9AC701AA1341AE7EF` (break `/Game/n00dComponents/n00dPacks/n00dGameplay/n00dSleeper/Blueprints/FN00dSleeper_Data` SleepDataForController)))
      (set `local.LocalSleepData` _array_element)
      (set `local.LocalFound` true)))
  ;[1 1 1] If we don't find a match, add it to the sleep data
  (if (not (`local.LocalFound`))
    (`KismetArrayLibrary.Array_Add` (`self.SleepData`) (`local.LocalSleepData`)))
  (bind _returnvalue (`GameplayStatics.SaveGameToSlot` self (`self.ServerSaveSlot`)))
  (return _returnvalue))

(fn `SaveServerSleepLocation`
  (params (ForController :type "Controller Object Reference") (Location :type "Vector Structure") (Rotation :type "Rotator Structure"))
  (returns (ReturnValue :type Boolean))
  (locals (LocalFound :type Boolean) (LocalSleepData :type "/Game/n00dComponents/n00dPacks/n00dGameplay/n00dSleeper/Blueprints/FN00dSleeper_Data Structure"))
  ;[1 1 1] Find the sleep data for this controller and set the location and rotation in its members
  (bind _sleepdata (message `/Game/n00dComponents/n00dPacks/n00dGameplay/n00dSleeper/Blueprints/BPI_N00dSleeper.GetSleepData` ForController))
  (for (_array_element _array_index) (`self.SleepData`)
    (if (== (`.SleeperGUID_16_625A7DD04788A2F9AC701AA1341AE7EF` (break `/Game/n00dComponents/n00dPacks/n00dGameplay/n00dSleeper/Blueprints/FN00dSleeper_Data` _array_element)) (`.SleeperGUID_16_625A7DD04788A2F9AC701AA1341AE7EF` (break `/Game/n00dComponents/n00dPacks/n00dGameplay/n00dSleeper/Blueprints/FN00dSleeper_Data` _sleepdata)))
      (set `local.LocalSleepData` _array_element)
      (set `local.LocalFound` true)))
  (if (`local.LocalFound`)
    (setmembers `/Game/n00dComponents/n00dPacks/n00dGameplay/n00dSleeper/Blueprints/FN00dSleeper_Data` :`StructRef` (`|GetArrayItem` (`self.SleepData`) _array_index) :`Location` Location :`Rotation` Rotation)
    ;[1 1 1] Save the new data to slot
    (bind _returnvalue (`GameplayStatics.SaveGameToSlot` self (`self.ServerSaveSlot`)))
    (return _returnvalue)))