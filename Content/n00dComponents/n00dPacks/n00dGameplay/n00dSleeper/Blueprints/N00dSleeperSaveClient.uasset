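; N00dSleeperSaveClient is a save game object that persists client-side data for the n00dSleeper system.
; It stores a sleeper GUID and a sleep data record, each set through its own save function.
; Each function updates its variable, immediately writes the object itself to the client save slot, and returns the save result.
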(fn `SaveClientSleepData`
  (params (SleepData :type "/Game/n00dComponents/n00dPacks/n00dGameplay/n00dSleeper/Blueprints/FN00dSleeper_Data Structure"))
  (returns (Saved :type Boolean))
  (`|ExecutionSequence`
    (:`then_0`
      (set `self.SavedSleepData` SleepData))
    (:`then_1`
      (bind _returnvalue (`GameplayStatics.SaveGameToSlot` self (`self.ClientSaveSlot`)))
      (return _returnvalue))))

(fn `SaveClientSleeperGUID`
  (params (SleeperGUID :type "Guid Structure"))
  (returns (SavedGUID :type Boolean))
  (set `self.ClientSleeperGUID` SleeperGUID)
  (bind _returnvalue (`GameplayStatics.SaveGameToSlot` self (`self.ClientSaveSlot`)))
  (return _returnvalue))