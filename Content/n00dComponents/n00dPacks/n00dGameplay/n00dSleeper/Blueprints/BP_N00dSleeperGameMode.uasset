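; Example game mode for the n00dSleeper system, forwarding player login, logout and initialisation to its BPC N00dSleeperGameMode component.
; Login handling waits one second for the client to spawn, and server sleeper data saves when play ends in the editor.
; ChoosePlayerStart prefers the player's sleeper actor, falling back to the first PlayerStart found.
; A getter exposes the component; the other sleeper getters are empty stubs.
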(event `self.ReceiveBeginPlay`
  (bind _bpc_n00dsleeper_gamemode (`self.BPC_N00dSleeper_GameMode`))
  ;[1 1 1] INTEGRATE ME
  ;;[1 1 1] Initialise
  (`parent.ReceiveBeginPlay`)
  (`/Game/n00dComponents/Core/N00dMasterComponent.Initialise` _bpc_n00dsleeper_gamemode (`/Game/n00dComponents/Core/N00dMasterComponent.Owning` _bpc_n00dsleeper_gamemode)))

(event `self.K2_PostLogin`
  (params (NewPlayer :type "PlayerController Object Reference"))
  ;[1 1 1] INTEGRATE ME
  ;;[1 1 1] Handle sleeper entry and exit
  (`parent.K2_PostLogin` NewPlayer)
  (`KismetSystemLibrary.Delay` 1.0) ; Short delay for client to be spawned . This cannot be avoided in BP
  (`/Game/n00dComponents/n00dPacks/n00dGameplay/n00dSleeper/Blueprints/BPC_N00dSleeper_GameMode.OnSleeperPostLogin` (`self.BPC_N00dSleeper_GameMode`) NewPlayer))

(event `self.K2_OnLogout`
  (params (ExitingController :type "Controller Object Reference"))
  ;[1 1 1] INTEGRATE ME
  ;;[1 1 1] Handle sleeper entry and exit
  (`parent.K2_OnLogout` ExitingController)
  (`/Game/n00dComponents/n00dPacks/n00dGameplay/n00dSleeper/Blueprints/BPC_N00dSleeper_GameMode.OnSleeperLogout` (`self.BPC_N00dSleeper_GameMode`) ExitingController))

(event `self.ReceiveEndPlay`
  (params (EndPlayReason :type "EEndPlayReason Enum" :default "Destroyed"))
  (switch `EEndPlayReason` EndPlayReason
    (:`EndPlayInEditor`
      (`/Game/n00dComponents/n00dPacks/n00dGameplay/n00dSleeper/Blueprints/BPC_N00dSleeper_GameMode.SaveServerSleeperData` (`self.BPC_N00dSleeper_GameMode`)))))

(fn `ChoosePlayerStart`
  (params (Player :type "Controller Object Reference"))
  (returns (ReturnValue :type "Actor Object Reference"))
  (bind _sleeperactor (`/Game/n00dComponents/n00dPacks/n00dGameplay/n00dSleeper/Blueprints/BPC_N00dSleeper_GameMode.ChooseSleeperStart` (`self.BPC_N00dSleeper_GameMode`) Player))
  ;[1 1 1] Override to get our desired player start (owner's sleeper actor)
  (`/Engine/EditorBlueprintResources/StandardMacros.IsValid` _sleeperactor
    (:`Is Valid`
      (return _sleeperactor) ; Return the sleeper actor
    )
    (:`Is Not Valid`
      ;[1 1 1] Loop the player starts and return the first one if there was no sleeper actor found for this controller. Swap this out for smarter ways to handle initial entry
      (bind _outactors (`GameplayStatics.GetAllActorsOfClass` "/Script/Engine.PlayerStart"))
      (for _array_element _outactors
        (return _array_element)))))

(fn `GetClientSleeperSave`
  (returns (ClientSave :type "/Game/n00dComponents/n00dPacks/n00dGameplay/n00dSleeper/Blueprints/BP_N00dSleeperSaveClient Object Reference"))
  (return null))

(fn `GetControllerSleeper`
  (returns (ControllerSleeperComponent :type "/Game/n00dComponents/n00dPacks/n00dGameplay/n00dSleeper/Blueprints/BPC_N00dSleeper_Controller Object Reference"))
  (return null))

(fn `GetGameModeSleeper`
  (returns (GameModeSleepComponent :type "/Game/n00dComponents/n00dPacks/n00dGameplay/n00dSleeper/Blueprints/BPC_N00dSleeper_GameMode Object Reference"))
  (return (`self.BPC_N00dSleeper_GameMode`)))

(fn `GetServerSleeperSave`
  (returns (ServerSave :type "/Game/n00dComponents/n00dPacks/n00dGameplay/n00dSleeper/Blueprints/BP_N00dSleeperSaveServer Object Reference"))
  (return null))

(fn `GetSleepData`
  (returns (SleepData :type "/Game/n00dComponents/n00dPacks/n00dGameplay/n00dSleeper/Blueprints/FN00dSleeper_Data Structure"))
  (return))

(fn `UserConstructionScript`
  (`parent.UserConstructionScript`))