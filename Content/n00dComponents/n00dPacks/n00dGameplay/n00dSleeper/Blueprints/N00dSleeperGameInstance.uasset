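; Game instance for the n00dSleeper system that keeps the client's sleep data and persistent sleeper GUID.
; On Init it loads the N00dSleeperSaveClient save from its slot, or creates and saves one.
; A valid saved GUID has its data copied to LoadedSleepData; otherwise a new GUID is saved without updating that copy.
; GetSleepData exposes the cached data to spare casts, while GetSleeperComponent is an empty stub.
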(event `self.ReceiveInit`
  ;[1 1 1] INTEGRATE ME
  ;;[0.09035 0.695 0.1803] Initialise
  (`self.LoadClientSleeperObject`)
  (`self.LoadClientSleeperData`))

(event `SaveClientSleeperObject`
  ;[1 1 1] INTEGRATE ME
  ;;[1 0.9455 0.1593] Serialisation
  ;;;[1 1 1] Save Client Sleeper Object
  (bind _returnvalue (`GameplayStatics.SaveGameToSlot` (`self.ClientSleeperSave`) (`self.SleeperSaveSlot`)))
  (if _returnvalue
    (`KismetSystemLibrary.PrintString` "Client SUCCEEDED in Saving Game to Slot" true true (struct :`R` 0.09035 :`G` 0.695 :`B` 0.180317 :`A` 1.0) 2.0)
    (else
      (`KismetSystemLibrary.PrintString` "Client FAILED to Save Game to Slot" true true (struct :`R` 1.0 :`G` 0.05 :`B` 0.05 :`A` 1.0) 10.0))))

(event `LoadClientSleeperObject`
  (bind _sleepersaveslot (`self.SleeperSaveSlot`))
  ;[1 1 1] INTEGRATE ME
  ;;[1 0.9455 0.1593] Serialisation
  ;;;[1 1 1] Load Client Sleeper Object
  (`/Engine/EditorBlueprintResources/StandardMacros.IsValid` (`self.ClientSleeperSave`)
    (:`Is Valid`
      _)
    (:`Is Not Valid`
      (bind _returnvalue (`GameplayStatics.CreateSaveGameObject` "/Game/n00dComponents/n00dPacks/n00dGameplay/n00dSleeper/Blueprints/N00dSleeperSaveClient.N00dSleeperSaveClient_C"))
      (set `self.ClientSleeperSave` _returnvalue)))
  (bind _returnvalue_2 (`GameplayStatics.DoesSaveGameExist` (`self.SleeperSaveSlot`)))
  (if _returnvalue_2
    (bind _returnvalue_3 (`GameplayStatics.LoadGameFromSlot` _sleepersaveslot))
    (bind _asn00d_sleeper_save_client (cast `/Game/n00dComponents/n00dPacks/n00dGameplay/n00dSleeper/Blueprints/N00dSleeperSaveClient` _returnvalue_3))
    (set `self.ClientSleeperSave` _asn00d_sleeper_save_client)
    (`KismetSystemLibrary.PrintString` "SUCCEEDED in Loading Client Game from Slot" true true (struct :`R` 0.09035 :`G` 0.695 :`B` 0.180317 :`A` 1.0))
    (else
      (bind _returnvalue_4 (`GameplayStatics.SaveGameToSlot` (`self.ClientSleeperSave`) _sleepersaveslot))
      (if _returnvalue_4
        (`KismetSystemLibrary.PrintString` "SUCCEEDED in Saving Client Game to Slot" true true (struct :`R` 0.09035 :`G` 0.695 :`B` 0.180317 :`A` 1.0))
        (else
          (`KismetSystemLibrary.PrintString` "FAILED to Save Client Game to Slot" true true (struct :`R` 1.0 :`G` 0.05 :`B` 0.05 :`A` 1.0) 10.0))))))

(event `LoadClientSleeperData`
  (bind _savedsleepdata (`/Game/n00dComponents/n00dPacks/n00dGameplay/n00dSleeper/Blueprints/N00dSleeperSaveClient.SavedSleepData` (`self.ClientSleeperSave`)))
  ;[1 1 1] INTEGRATE ME
  ;;[1 0.9455 0.1593] Serialisation
  ;;;[1 1 1] Load Client Sleeper GUID from Save
  (if (`KismetGuidLibrary.IsValid_Guid` (`.SleeperGUID_16_625A7DD04788A2F9AC701AA1341AE7EF` (break `/Game/n00dComponents/n00dPacks/n00dGameplay/n00dSleeper/Blueprints/FN00dSleeper_Data` _savedsleepdata)))
    (set `self.LoadedSleepData` _savedsleepdata) ; Load the sleep data if the GUID is valid
    (`KismetSystemLibrary.PrintString` "Sleep Data LOADED on the GameInstance" true true (struct :`R` 0.09035 :`G` 0.695 :`B` 0.180317 :`A` 1.0))
    (else
      (bind _structout (setmembers `/Game/n00dComponents/n00dPacks/n00dGameplay/n00dSleeper/Blueprints/FN00dSleeper_Data` :`StructRef` (`/Game/n00dComponents/n00dPacks/n00dGameplay/n00dSleeper/Blueprints/N00dSleeperSaveClient.SavedSleepData` (`self.ClientSleeperSave`)) :`SleeperGUID` (`KismetGuidLibrary.NewGuid`)))
      (bind _saved (`/Game/n00dComponents/n00dPacks/n00dGameplay/n00dSleeper/Blueprints/N00dSleeperSaveClient.SaveClientSleepData` (`self.ClientSleeperSave`) _structout))
      (if _saved
        (`KismetSystemLibrary.PrintString` "Sleep Data SAVED on the GameInstance" true true (struct :`R` 0.09035 :`G` 0.695 :`B` 0.180317 :`A` 1.0))
        (else
          (`KismetSystemLibrary.PrintString` "Sleep Data FAILED to save on the GameInstance" true true (struct :`R` 1.0 :`G` 0.05 :`B` 0.05 :`A` 1.0) 10.0))))))

(fn `GetSleepData`
  (returns (SleepData :type "/Game/n00dComponents/n00dPacks/n00dGameplay/n00dSleeper/Blueprints/FN00dSleeper_Data Structure"))
  ;[1 1 1] Calling this avoids a cast in other BPs
  (return (`self.LoadedSleepData`)))

(fn `GetSleeperComponent`
  (returns (SleeperComponent :type "/Game/n00dComponents/n00dPacks/n00dGameplay/n00dSleeper/Blueprints/BPC_N00dSleeper Object Reference"))
  (return null))