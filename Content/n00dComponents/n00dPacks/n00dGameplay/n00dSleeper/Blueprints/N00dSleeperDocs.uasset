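; N00dSleeperDocs is a documentation Blueprint in the n00dSleeper pack that displays a logo card and stores a link.
; Its construction script applies the configured scale and sprite to the LogoCard component.
; It then sets DocumentLink from the Discord link or the website link based on two booleans, with Discord taking priority and the value left unchanged if neither is set.
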(fn `UserConstructionScript`
  ;[1 1 1] Construct scale and texture
  (`SceneComponent.SetRelativeScale3D` (`self.LogoCard`) (`self.LogoScale`))
  (`BillboardComponent.SetSprite` (`self.LogoCard`) (`self.Logo`))
  ;[1 1 1] Set the link according to our bool
  (if (`self.IsDiscord`)
    (set `self.DocumentLink` (`KismetTextLibrary.Conv_TextToString` (`self.DiscordLink`)))
    (elif (`self.IsWebsite`)
      (set `self.DocumentLink` (`KismetTextLibrary.Conv_TextToString` (`self.WebsiteLink`))))))