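; Player controller that hosts the n00dSleeper component, with setup marked for copying.
; Construction applies component defaults; BeginPlay passes controller and possessed Character mesh references into the component's Initialise.
; It forwards server SleepData from the GameMode for debug and security comparison, and exposes the component and loaded data through getters.
; Debug keys O and I open a listen-server session or connect to a hardcoded local address.
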(event `self.ReceiveBeginPlay`
  (bind _bpc_n00dsleeper (`self.BPC_N00dSleeper`))
  (`parent.ReceiveBeginPlay`)
  ;[1 1 1] COPY ME
  ;;[1 1 1] Initialise Sleeper for Controller
  (bind _ascharacter (cast `Character` (`self.K2_GetPawn`)))
  (bind _structout (setmembers `/Game/n00dComponents/Core/FOwning` :`StructRef` (`/Game/n00dComponents/Core/N00dMasterComponent.Owning` _bpc_n00dsleeper) :`Controller` self :`PlayerController` self :`SkeletalMesh` (`Character.Mesh` _ascharacter)))
  (`/Game/n00dComponents/Core/N00dMasterComponent.Initialise` _bpc_n00dsleeper _structout))

(event `Key|O`
  (params (Key :type "Key Structure" :default "AnyKey"))
  ;[1 1 1] COPY ME
  ;;[1 1 1] DEBUG - GameInstance needs to be applied in Migrate Project
  ;;;[1 1 1] Open a Listen server session (make sure to delete N00dDocs from map before building as it tries to call Billboard before its created)
  (:`Pressed`
    (`/Game/n00dComponents/n00dPacks/n00dGameplay/n00dSleeper/Blueprints/BPC_N00dSleeper.DebugOpenSleeperSession` (`self.BPC_N00dSleeper`))))

(event `Key|I`
  (params (Key :type "Key Structure" :default "AnyKey"))
  ;[1 1 1] COPY ME
  ;;[1 1 1] DEBUG - GameInstance needs to be applied in Migrate Project
  ;;;[1 1 1] Open a local connection to a listen server
  (:`Pressed`
    (`/Game/n00dComponents/n00dPacks/n00dGameplay/n00dSleeper/Blueprints/BPC_N00dSleeper.DebugConnectSleeperSession` (`self.BPC_N00dSleeper`) "192.168.1.18:7777")))

(event `/Game/n00dComponents/n00dPacks/n00dGameplay/n00dSleeper/Blueprints/BPI_N00dSleeper.SetSleepData`
  (params (SleepData :type "/Game/n00dComponents/n00dPacks/n00dGameplay/n00dSleeper/Blueprints/FN00dSleeper_Data Structure"))
  ;[1 1 1] COPY ME
  ;;[1 1 1] Sent from Game Mode as Server SleepData - for debug and security compare
  (`/Game/n00dComponents/n00dPacks/n00dGameplay/n00dSleeper/Blueprints/BPC_N00dSleeper.OwningSleepDataFromServer` (`self.BPC_N00dSleeper`) SleepData))

(fn `GetSleepData`
  (returns (SleepData :type "/Game/n00dComponents/n00dPacks/n00dGameplay/n00dSleeper/Blueprints/FN00dSleeper_Data Structure"))
  ;[1 1 1] Parse the component's sleep data to BPI_N00dSleeper
  (return (`/Game/n00dComponents/n00dPacks/n00dGameplay/n00dSleeper/Blueprints/BPC_N00dSleeper.LoadedSleepData` (`self.BPC_N00dSleeper`))))

(fn `GetSleeperComponent`
  (returns (SleeperComponent :type "/Game/n00dComponents/n00dPacks/n00dGameplay/n00dSleeper/Blueprints/BPC_N00dSleeper Object Reference"))
  ;[1 1 1] Get sleeper component
  (return (`self.BPC_N00dSleeper`)))

(fn `UserConstructionScript`
  ;[1 1 1] Set the component animations in the loaded sleep data
  (`parent.UserConstructionScript`)
  (`/Game/n00dComponents/n00dPacks/n00dGameplay/n00dSleeper/Blueprints/BPC_N00dSleeper.ConstructDefaults` (`self.BPC_N00dSleeper`)))