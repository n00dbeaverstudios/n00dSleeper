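; Example character for the n00dSleeper system, whose event logic is marked for integration.
; It passes its mesh and movement component to BPCN00dSleeperCharacter on BeginPlay.
; Visibility changes from the sleeper actor run on authority, where the component multicasts mesh visibility and handles movement disabling.
; A debug Tab key rebuilds a HUD list of all sleeper actors; the sleeper getter functions are empty stubs.
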(event `/Game/n00dComponents/n00dPacks/n00dGameplay/n00dSleeper/Blueprints/BPI_N00dSleeper.SetSleeperVisibility`
  (params (NewVisibility :type Boolean) (DisableMovement :type Boolean))
  (bind _bpc_n00dsleeper_character (`self.BPC_N00dSleeper_Character`))
  ;[1 1 1] INTEGRATE ME
  ;;[0.1903 0.6116 0.705] Set sleeper visibility and movement from server (this comes from the sleeper actor)
  (`/Engine/EditorBlueprintResources/ActorMacros.Switch Has Authority`
    (:`Authority`
      (`/Game/n00dComponents/n00dPacks/n00dGameplay/n00dSleeper/Blueprints/BPC_N00dSleeper_Character.MulticastMeshVisibility` _bpc_n00dsleeper_character NewVisibility)
      (`/Game/n00dComponents/n00dPacks/n00dGameplay/n00dSleeper/Blueprints/BPC_N00dSleeper_Character.HandleMovement` _bpc_n00dsleeper_character DisableMovement))))

(event `self.ReceiveBeginPlay`
  (bind _bpc_n00dsleeper_character (`self.BPC_N00dSleeper_Character`))
  ;[1 1 1] INTEGRATE ME
  ;;[0.09035 0.695 0.1803] Initialise
  (`parent.ReceiveBeginPlay`)
  ;;[0.09035 0.695 0.1803] Send necessary references to the component
  (bind _structout (setmembers `/Game/n00dComponents/Core/FOwning` :`StructRef` (`/Game/n00dComponents/Core/N00dMasterComponent.Owning` _bpc_n00dsleeper_character) :`SkeletalMesh` (`self.Mesh`) :`CMC` (`self.CharacterMovement`)))
  (`/Game/n00dComponents/Core/N00dMasterComponent.Initialise` _bpc_n00dsleeper_character _structout))

(event `Key|Tab`
  (params (Key :type "Key Structure" :default "AnyKey"))
  ;[0.2462 0.323 0.34] DEBUG: Add or remove active or inactive sleep actors on HUD list - only works in the n00dCharacter class
  (:`Pressed`
    (`PanelWidget.ClearChildren` (`/Game/n00dComponents/n00dPacks/n00dGameplay/n00dSleeper/Blueprints/WBP_N00dSleeper_HUD.ActiveActorsContainer` (cast `/Game/n00dComponents/n00dPacks/n00dGameplay/n00dSleeper/Blueprints/WBP_N00dSleeper_HUD` (`self.SpawnedHUD`) :!pure true)))
    (bind _outactors (`GameplayStatics.GetAllActorsOfClass` "/Game/n00dComponents/n00dPacks/n00dGameplay/n00dSleeper/Blueprints/BP_N00dSleeperActor.BP_N00dSleeperActor_C"))
    (for _array_element _outactors
      (bind _returnvalue (`|CreateWidget` "/Game/n00dComponents/n00dPacks/n00dGameplay/n00dSleeper/Blueprints/WBP_N00dSleeper_Debug.WBP_N00dSleeper_Debug_C" (cast `PlayerController` (`self.GetController`) :!pure true) (`KismetTextLibrary.Conv_StringToText` (`KismetSystemLibrary.GetObjectName` _array_element))))
      (`PanelWidget.AddChild` (`/Game/n00dComponents/n00dPacks/n00dGameplay/n00dSleeper/Blueprints/WBP_N00dSleeper_HUD.ActiveActorsContainer` (cast `/Game/n00dComponents/n00dPacks/n00dGameplay/n00dSleeper/Blueprints/WBP_N00dSleeper_HUD` (`self.SpawnedHUD`) :!pure true)) _returnvalue))))

(fn `GetClientSleeperSave`
  (returns (ClientSave :type "/Game/n00dComponents/n00dPacks/n00dGameplay/n00dSleeper/Blueprints/BP_N00dSleeperSaveClient Object Reference"))
  (return null))

(fn `GetControllerSleeper`
  (returns (ControllerSleeperComponent :type "/Game/n00dComponents/n00dPacks/n00dGameplay/n00dSleeper/Blueprints/BPC_N00dSleeper_Controller Object Reference"))
  (return null))

(fn `GetGameModeSleeper`
  (returns (GameModeSleepComponent :type "/Game/n00dComponents/n00dPacks/n00dGameplay/n00dSleeper/Blueprints/BPC_N00dSleeper_GameMode Object Reference"))
  (return null))

(fn `GetServerSleeperSave`
  (returns (ServerSave :type "/Game/n00dComponents/n00dPacks/n00dGameplay/n00dSleeper/Blueprints/BP_N00dSleeperSaveServer Object Reference"))
  (return null))

(fn `GetSleepData`
  (returns (SleepData :type "/Game/n00dComponents/n00dPacks/n00dGameplay/n00dSleeper/Blueprints/FN00dSleeper_Data Structure"))
  (return))

(fn `UserConstructionScript`
  (`parent.UserConstructionScript`))