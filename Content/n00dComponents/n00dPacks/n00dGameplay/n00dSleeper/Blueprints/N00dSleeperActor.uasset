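; Replicated sleeper actor that stands in as a sleeping body, playing fall-asleep, sleep-loop and wake-up animations and sounds from a sleep data struct.
; The server multicasts the one-shot transitions, while mesh, loop animation and loop sound use OnRep variables so they stay relevant.
; Falling asleep starts the loop after the transition's length.
; Waking hides and freezes the controlled pawn, then after the animation restores it and asks the GameMode's sleeper component to remove this actor.
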(event `MulticastSleep`
  (params (Animation :type "AnimSequence Object Reference") (Sound :type "SoundBase Object Reference"))
  (bind _transitionaudiocomponent (`self.TransitionAudioComponent`))
  ;[0.1903 0.6116 0.705] Network
  ;;[1 1 1] Multicast the transition sleep animations and sounds
  (`SkeletalMeshComponent.PlayAnimation` (`self.SleeperMeshComponent`) Animation false)
  (`AudioComponent.SetSound` _transitionaudiocomponent Sound)
  (`AudioComponent.Play` _transitionaudiocomponent 0.0))

(event `SleepLoop`
  (params (Delay :type "Float (double-precision)") (LoopAnimation :type "AnimSequence Object Reference") (LoopSound :type "SoundBase Object Reference"))
  ;[0.1903 0.6116 0.705] Network
  ;;[1 1 1] OnRep the Sleep Loop after a delay
  (`KismetSystemLibrary.Delay` Delay)
  (set `self.SleepLoopAnim` LoopAnimation)
  (set `self.LoopSound` LoopSound))

(event `WakeUpDelay`
  (params (Delay :type "Float (double-precision)") (ForController :type "Controller Object Reference"))
  ;[0.1903 0.6116 0.705] Network
  ;;[1 1 1] Return movement to the character once the delay is complete and destroy the actor
  (`KismetSystemLibrary.Delay` Delay)
  (message `/Game/n00dComponents/n00dPacks/n00dGameplay/n00dSleeper/Blueprints/BPI_N00dSleeper.SetSleeperVisibility` (`Controller.K2_GetPawn` ForController) true false)
  (bind _sleepercomponent (message `/Game/n00dComponents/n00dPacks/n00dGameplay/n00dSleeper/Blueprints/BPI_N00dSleeper.GetSleeperComponent` (`GameplayStatics.GetGameMode`)))
  (`/Game/n00dComponents/n00dPacks/n00dGameplay/n00dSleeper/Blueprints/BPC_N00dSleeper.RemoveSleepActor` _sleepercomponent self))

(fn `FallAsleep`
  (params (SleepData :type "/Game/n00dComponents/n00dPacks/n00dGameplay/n00dSleeper/Blueprints/FN00dSleeper_Data Structure"))
  (bind ((`Animations_23_0C71528045C90A61DD4D64B48A4F1F75` _animations) (`Sounds_32_0ED13F04442334FEB05781AA7C0F27EC` _sounds)) (break `/Game/n00dComponents/n00dPacks/n00dGameplay/n00dSleeper/Blueprints/FN00dSleeper_Data` (`self.SleepData`)))
  (bind ((`ToSleep_2_EFF671844CD5F3AE8B2A2F90D7675857` _tosleep) (`SleepLoop_4_B3B2782043C00FB1EA8BE0BEDF8F1336` _sleeploop)) (break `/Game/n00dComponents/n00dPacks/n00dGameplay/n00dSleeper/Blueprints/FN00dSleeper_Animation` _animations))
  (`/Engine/EditorBlueprintResources/ActorMacros.Switch Has Authority`
    (:`Authority`
      ;[1 1 1] Cache data and set an OnRep mesh change
      (bind _output_get (set `self.SleepData` SleepData))
      (bind ((`SkeletalMesh_2_5D89AE164E23AED409603286CD9583A3` _skeletalmesh) (`Animations_23_0C71528045C90A61DD4D64B48A4F1F75` _animations_2) (`Sounds_32_0ED13F04442334FEB05781AA7C0F27EC` _sounds_2)) (break `/Game/n00dComponents/n00dPacks/n00dGameplay/n00dSleeper/Blueprints/FN00dSleeper_Data` _output_get))
      (set `self.SleeperMesh` _skeletalmesh)
      (`self.MulticastSleep` (`.ToSleep_2_EFF671844CD5F3AE8B2A2F90D7675857` (break `/Game/n00dComponents/n00dPacks/n00dGameplay/n00dSleeper/Blueprints/FN00dSleeper_Animation` _animations_2)) (`.ToSleep_2_04876C7F41700C16BB42A3A4DA65422C` (break `/Game/n00dComponents/n00dPacks/n00dGameplay/n00dSleeper/Blueprints/FN00dSleeper_Sounds` _sounds_2))) ; Only multicast ToSleep as we don't need it to be relevant
      ;[1 1 1] Handle play length and sleep loop
      (bind _returnvalue (`AnimSequenceBase.GetPlayLength` _tosleep))
      (`self.SleepLoop` _returnvalue _sleeploop (`.SleepLoop_4_653B2443495E4FA521BBA59B2E8ABD07` (break `/Game/n00dComponents/n00dPacks/n00dGameplay/n00dSleeper/Blueprints/FN00dSleeper_Sounds` _sounds)))
      (return))
    (:`Remote`
      (return))))

(fn `GetSleepData`
  (returns (SleepData :type "/Game/n00dComponents/n00dPacks/n00dGameplay/n00dSleeper/Blueprints/FN00dSleeper_Data Structure"))
  ;[1 1 1] Parse the actor sleep data to the interface
  (return (`self.SleepData`)))

(fn `GetSleeperComponent`
  (returns (SleeperComponent :type "/Game/n00dComponents/n00dPacks/n00dGameplay/n00dSleeper/Blueprints/BPC_N00dSleeper Object Reference"))
  (return null))

(fn `OnRep_LoopSound`
  (bind _loopsound (`self.LoopSound`))
  (bind _loopedaudiocomponent (`self.LoopedAudioComponent`))
  ;[1 1 1] Set the sound and play it
  (`AudioComponent.SetSound` _loopedaudiocomponent _loopsound)
  (`/Engine/EditorBlueprintResources/StandardMacros.IsValid` _loopsound
    (:`Is Valid`
      (`AudioComponent.Play` _loopedaudiocomponent 0.0))
    (:`Is Not Valid`
      (`AudioComponent.Stop` _loopedaudiocomponent)))
  (return))

(fn `OnRep_SleeperMesh`
  ;[1 1 1] Set the actor mesh from the controller sleep data
  (`SkinnedMeshComponent.SetSkinnedAssetAndUpdate` (`self.SleeperMeshComponent`) (`.SkeletalMesh_2_5D89AE164E23AED409603286CD9583A3` (break `/Game/n00dComponents/n00dPacks/n00dGameplay/n00dSleeper/Blueprints/FN00dSleeper_Data` (`self.SleepData`))) true)
  (return))

(fn `OnRep_SleepLoopAnim`
  ;[1 1 1] Play SleepLoop
  (`SkeletalMeshComponent.PlayAnimation` (`self.SleeperMeshComponent`) (`self.SleepLoopAnim`) true)
  (return))

(fn `UserConstructionScript`)

(fn `WakeUp`
  (params (Controller :type "Controller Object Reference"))
  (locals (LocalPlayLength :type "Float (double-precision)"))
  (`/Engine/EditorBlueprintResources/ActorMacros.Switch Has Authority`
    (:`Authority`
      ;[1 1 1] Get the sleep data from the controller
      (bind _output_get (set `self.OwningSleeperController` Controller))
      (bind _sleepdata (message `/Game/n00dComponents/n00dPacks/n00dGameplay/n00dSleeper/Blueprints/BPI_N00dSleeper.GetSleepData` _output_get))
      ;[1 1 1] Set the sleep data, multicast the mesh visibility and the FROM SLEEP animation, and get the play length
      (bind _output_get_2 (set `self.SleepData` _sleepdata))
      (message `/Game/n00dComponents/n00dPacks/n00dGameplay/n00dSleeper/Blueprints/BPI_N00dSleeper.SetSleeperVisibility` (`Controller.K2_GetPawn` _output_get) false true)
      (set `self.LoopSound` null) ; Clear the looped sound
      (bind ((`SkeletalMesh_2_5D89AE164E23AED409603286CD9583A3` _skeletalmesh) (`Animations_23_0C71528045C90A61DD4D64B48A4F1F75` _animations) (`Sounds_32_0ED13F04442334FEB05781AA7C0F27EC` _sounds)) (break `/Game/n00dComponents/n00dPacks/n00dGameplay/n00dSleeper/Blueprints/FN00dSleeper_Data` _output_get_2))
      (bind ((`FromSleep_6_BE4A8AAA4058BC40F7E3B995B7FC0BD9` _fromsleep)) (break `/Game/n00dComponents/n00dPacks/n00dGameplay/n00dSleeper/Blueprints/FN00dSleeper_Animation` _animations))
      (`self.MulticastSleep` _fromsleep (`.FromSleep_6_703A78734A0CA14774E26D8440FF25B8` (break `/Game/n00dComponents/n00dPacks/n00dGameplay/n00dSleeper/Blueprints/FN00dSleeper_Sounds` _sounds))) ; Only multicast FromSleep as we don't need it to be relevant
      (bind _returnvalue (`AnimSequenceBase.GetPlayLength` _fromsleep))
      (set `local.LocalPlayLength` _returnvalue)
      ;[1 1 1] Send to a delayed event
      (`self.WakeUpDelay` (`local.LocalPlayLength`) (`self.OwningSleeperController`)))
    (:`Remote`
      (return))))