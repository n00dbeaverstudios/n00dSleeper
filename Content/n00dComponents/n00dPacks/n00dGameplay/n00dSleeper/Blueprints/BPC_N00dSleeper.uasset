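; n00d Sleeper component that leaves a sleeping body in the world when a player logs out and wakes it on return.
; One component serves both GameMode and Controller, choosing its setup by an owner-type enum.
; The GameMode side loads a server SaveGame, respawns sleep actors, and matches players to them by GUID at login and logout.
; The Controller side passes the GameInstance's GUID to the server and optionally fades vision in from black.
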(event `DeleteSave`
  ;[1 0.05 0.05] Delete the sleeper saves for client and server
  (`self.DeleteServerSleepData`)
  (`self.DeleteClientSleepData`))

(event `self.Initialise`
  (params (Owning :type "/Game/n00dComponents/Core/FOwning Structure"))
  ;[1 1 1] Initialise
  (`parent.Initialise` Owning)
  ;[1 1 1] Since this component is intended to be attached to multiple different systems at once, we need to check who the owner is before initialising this instance of the component. Static variables are much cheaper than casting to find the owner
  (switch `/Game/n00dComponents/n00dPacks/n00dGameplay/n00dSleeper/Blueprints/EN00dSleeper_OwningActor` (`self.OwningActorType`) ; What actor is this component intended for
    (:`NewEnumerator0`
      ;;[0.09035 0.695 0.1803] Initialise for Owner
      (`self.GameModeInitialise`))
    (:`NewEnumerator2`
      (`self.ControllerInitialise`))))

(event `ServerSetSleeperGUID`
  (params (SleeperGUID :type "Guid Structure"))
  ;[0.1903 0.6116 0.705] NETWORKING
  ;;[1 1 1] Set the GUID on the server so that the game mode can read it
  (`self.SetControllerSleepDataGUID` SleeperGUID))

(event `MulticastMeshVisibility`
  (params (bNewVisibility :type Boolean))
  ;[0.1903 0.6116 0.705] NETWORKING
  ;;[1 1 1] Multicast the character mesh visibilities
  ;; Called from the sleep actor, sent from Character
  (`SceneComponent.SetVisibility` (`self.OwningSkeletalMesh`) bNewVisibility true))

(event `OwningSleepDataFromServer`
  (params (SleepData :type "/Game/n00dComponents/n00dPacks/n00dGameplay/n00dSleeper/Blueprints/FN00dSleeper_Data Structure"))
  ;[0.1903 0.6116 0.705] NETWORKING
  ;;[1 1 1] Set from Game Mode (server)
  ;;;[1 1 1] Owning debug sleep data
  (bind _output_get (set `self.DebugServerSleepData` SleepData))
  ;;;[0.2462 0.323 0.34] DEBUG
  (`self.Debug` "Debug Server Sleep Data GUID:" "NewEnumerator2" (`KismetGuidLibrary.Conv_GuidToString` (`.SleeperGUID_16_625A7DD04788A2F9AC701AA1341AE7EF` (break `/Game/n00dComponents/n00dPacks/n00dGameplay/n00dSleeper/Blueprints/FN00dSleeper_Data` _output_get)))))

(event `ServerSetLoadedSleepData`
  (params (SleepData :type "/Game/n00dComponents/n00dPacks/n00dGameplay/n00dSleeper/Blueprints/FN00dSleeper_Data Structure"))
  ;[0.1903 0.6116 0.705] NETWORKING
  ;;[1 1 1] Set from Game Instance (client)
  ;;;[1 1 1] Server Set SleepData
  (bind _output_get (set `self.LoadedSleepData` SleepData))
  ;;;[0.2462 0.323 0.34] DEBUG
  (`self.Debug` "LOADED SleepData for Controller GUID:" "NewEnumerator2" (`KismetGuidLibrary.Conv_GuidToString` (`.SleeperGUID_16_625A7DD04788A2F9AC701AA1341AE7EF` (break `/Game/n00dComponents/n00dPacks/n00dGameplay/n00dSleeper/Blueprints/FN00dSleeper_Data` _output_get))) false true 10.0))

(fn `AddPlayerToSleeperArray`
  (params (ForController :type "Controller Object Reference"))
  (bind (_location _yaw) (`self.ResolveSleeperWorldPositioning` ForController))
  (bind _sleepdata (message `/Game/n00dComponents/n00dPacks/n00dGameplay/n00dSleeper/Blueprints/BPI_N00dSleeper.GetSleepData` ForController))
  (if (`KismetGuidLibrary.IsValid_Guid` (`.SleeperGUID_16_625A7DD04788A2F9AC701AA1341AE7EF` (break `/Game/n00dComponents/n00dPacks/n00dGameplay/n00dSleeper/Blueprints/FN00dSleeper_Data` _sleepdata)))
    (bind _returnvalue (`KismetArrayLibrary.Array_Add` (`self.LoadedServerSleepData`) _sleepdata))
    (bind _output (`|GetArrayItem` (`self.LoadedServerSleepData`) _returnvalue))
    ;[1 1 1] Set the Sleep Actor index in the player's sleep data
    (setmembers `/Game/n00dComponents/n00dPacks/n00dGameplay/n00dSleeper/Blueprints/FN00dSleeper_Data` :`StructRef` _output :`SleepActorIndex` (`.SleepActorIndex_20_43AFEB9740D88D28FA4A2D80BC7285DA` (break `/Game/n00dComponents/n00dPacks/n00dGameplay/n00dSleeper/Blueprints/FN00dSleeper_Data` _output)) :`Location` _location :`Rotation` (`KismetMathLibrary.MakeRotator` 0.0 0.0 _yaw))
    (`self.SaveLoadedServerSleeperData`)
    (return)
    (else
      ;[1 1 1] DEBUG
      (`self.Debug` "Controller GUID Not Valid when ADDING PLAYER TO ARRAY" "NewEnumerator0")
      (return))))

(fn `AddToActiveSleeperActors`
  (params (SleeperActor :type "/Game/n00dComponents/n00dPacks/n00dGameplay/n00dSleeper/Blueprints/N00dSleeperActor Object Reference (by ref)") (ForController :type "Controller Object Reference") (SleepDataIndex :type Integer) (SleepActorIndex :type Integer))
  (locals (LocalSleeper :type "/Game/n00dComponents/n00dPacks/n00dGameplay/n00dSleeper/Blueprints/N00dSleeperActor Object Reference") (LocalController :type "Controller Object Reference") (LocalActorIndex :type Integer) (LocalDataIndex :type Integer))
  (bind _sleepdata (`/Game/n00dComponents/n00dPacks/n00dGameplay/n00dSleeper/Blueprints/N00dSleeperSaveServer.SleepData` (`self.SleeperSaveServer`)))
  ;[1 1 1] Cache
  (set `local.LocalSleeper` SleeperActor)
  (set `local.LocalController` ForController)
  (set `local.LocalDataIndex` SleepDataIndex)
  (set `local.LocalActorIndex` SleepActorIndex)
  (`/Engine/EditorBlueprintResources/StandardMacros.IsValid` (`local.LocalController`) ; Have we got an incoming controller
    (:`Is Valid`
      ;[1 1 1] If there is an active controller, lets save its sleep actor index on the server data for this controller. It means we're logging out (sleeping)
      (bind _returnvalue (`KismetArrayLibrary.Array_Add` (`self.ActiveSleepActors`) (`local.LocalSleeper`)))
      (bind _sleepdata_2 (message `/Game/n00dComponents/n00dPacks/n00dGameplay/n00dSleeper/Blueprints/BPI_N00dSleeper.GetSleepData` (`local.LocalController`))) ; Grab the sleep data from the controller
      ;;[0.2462 0.323 0.34] DEBUG
      (`self.Debug` "New ACTIVE SLEEPER: Index" "NewEnumerator2" (`KismetStringLibrary.Conv_IntToString` _returnvalue) false true 10.0)
      (bind ((`Animations_23_0C71528045C90A61DD4D64B48A4F1F75` _animations) (`Sounds_32_0ED13F04442334FEB05781AA7C0F27EC` _sounds) (`SleeperGUID_16_625A7DD04788A2F9AC701AA1341AE7EF` _sleeperguid)) (break `/Game/n00dComponents/n00dPacks/n00dGameplay/n00dSleeper/Blueprints/FN00dSleeper_Data` _sleepdata_2))
      ;;[1 1 1] Set the sleep actor index in the member of the server sleep data
      (setmembers `/Game/n00dComponents/n00dPacks/n00dGameplay/n00dSleeper/Blueprints/FN00dSleeper_Data` :`StructRef` (`|GetArrayItem` _sleepdata (+ (`KismetArrayLibrary.Array_Find` _sleepdata _sleepdata_2) 1)) :`Animations` _animations :`Sounds` _sounds :`SleeperGUID` _sleeperguid :`SleepActorIndex` _returnvalue)
      (`self.SaveLoadedServerSleeperData`)
      (return))
    (:`Is Not Valid`
      ;[1 1 1] If the controller is not valid that means we're loading the server, so set the index from the save and reference the actor in the active list - this willl be looping
      ;;[1 1 1] ...and map the actor index to the sleep data index the same as it was when saved
      (setmembers `/Game/n00dComponents/n00dPacks/n00dGameplay/n00dSleeper/Blueprints/FN00dSleeper_Data` :`StructRef` (`|GetArrayItem` (`/Game/n00dComponents/n00dPacks/n00dGameplay/n00dSleeper/Blueprints/N00dSleeperSaveServer.SleepData` (`self.SleeperSaveServer`)) (`local.LocalDataIndex`)) :`SleepActorIndex` (`local.LocalActorIndex`))
      ;;[1 1 1] Set array on the specified index (create array the same as it was)
      (`KismetArrayLibrary.Array_Set` (`self.ActiveSleepActors`) (`local.LocalActorIndex`) (`local.LocalSleeper`) true)
      (return))))

(fn `CachePlayerSleepData`
  (params (ForController :type "Controller Object Reference"))
  (returns (Added :type Boolean))
  (locals (LocalSleepData :type "/Game/n00dComponents/n00dPacks/n00dGameplay/n00dSleeper/Blueprints/FN00dSleeper_Data Structure") (LocalSleeperForControllerGUID :type "Guid Structure") (LocalExisitingGUID :type Boolean) (LocalForController :type "Controller Object Reference"))
  (bind _loadedserversleepdata (`self.LoadedServerSleepData`))
  ;[1 1 1] Cache the client values
  (bind _output_get (set `local.LocalForController` ForController))
  (bind _sleepdata (message `/Game/n00dComponents/n00dPacks/n00dGameplay/n00dSleeper/Blueprints/BPI_N00dSleeper.GetSleepData` _output_get))
  (set `local.LocalSleepData` _sleepdata)
  (set `local.LocalSleeperForControllerGUID` (`.SleeperGUID_16_625A7DD04788A2F9AC701AA1341AE7EF` (break `/Game/n00dComponents/n00dPacks/n00dGameplay/n00dSleeper/Blueprints/FN00dSleeper_Data` _sleepdata)))
  ;[1 1 1] Look for the incoming GUID in the server array and see if it matches the incoming. Mark it as existing if we find one
  (for _array_element (`self.LoadedServerSleepData`)
    (if (== (`local.LocalSleeperForControllerGUID`) (`.SleeperGUID_16_625A7DD04788A2F9AC701AA1341AE7EF` (break `/Game/n00dComponents/n00dPacks/n00dGameplay/n00dSleeper/Blueprints/FN00dSleeper_Data` _array_element)))
      (set `local.LocalExisitingGUID` true)))
  ;[1 1 1] @TODO
  ;;[1 1 1] Just return if found, otherwise do the thing...
  (if (not (`local.LocalExisitingGUID`))
    ;;;[1 1 1] Add the controller's sleep data to the server and save the data to disk
    (bind _returnvalue (`KismetArrayLibrary.Array_Add` _loadedserversleepdata (`local.LocalSleepData`)))
    (setmembers `/Game/n00dComponents/n00dPacks/n00dGameplay/n00dSleeper/Blueprints/FN00dSleeper_Data` :`StructRef` (`|GetArrayItem` _loadedserversleepdata _returnvalue) :`SleeperGUID` (`local.LocalSleeperForControllerGUID`) :`SleepActorIndex` (`.SleepActorIndex_20_43AFEB9740D88D28FA4A2D80BC7285DA` (break `/Game/n00dComponents/n00dPacks/n00dGameplay/n00dSleeper/Blueprints/FN00dSleeper_Data` _sleepdata))) ; and set the controller's GUID within
    (bind _saved (`/Game/n00dComponents/n00dPacks/n00dGameplay/n00dSleeper/Blueprints/N00dSleeperSaveServer.SaveServerGameModeSleeperData` (`self.SleeperSaveServer`) _loadedserversleepdata))
    (`KismetSystemLibrary.PrintString` (`KismetStringLibrary.Concat_StrStr` "SAVED SERVER DATA " (`KismetStringLibrary.Conv_BoolToString` _saved)) true true (struct :`R` 1.0 :`G` 0.05 :`B` 0.05 :`A` 1.0) 10.0))
  (return (`local.LocalExisitingGUID`)))

(fn `ChooseSleeperStart`
  (params (ForController :type "Controller Object Reference"))
  (returns (SleeperActor :type "/Game/n00dComponents/n00dPacks/n00dGameplay/n00dSleeper/Blueprints/N00dSleeperActor Object Reference"))
  ;[1 1 1] Return the actor at the controller's sleep index
  (return (`|GetArrayItem` (`self.ActiveSleepActors`) (`.SleepActorIndex_20_43AFEB9740D88D28FA4A2D80BC7285DA` (break `/Game/n00dComponents/n00dPacks/n00dGameplay/n00dSleeper/Blueprints/FN00dSleeper_Data` (`self.GetSleepDataFromServerSave` ForController))))))

(fn `ConstructDefaults`
  (bind (_sleepsounds_tosleep _sleepsounds_sleeploop _sleepsounds_fromsleep) (break `/Game/n00dComponents/n00dPacks/n00dGameplay/n00dSleeper/Blueprints/FN00dSleeper_Sounds` (`self.SleepSounds`)))
  (bind (_sleepanimations_tosleep _sleepanimations_sleeploop _sleepanimations_fromsleep) (break `/Game/n00dComponents/n00dPacks/n00dGameplay/n00dSleeper/Blueprints/FN00dSleeper_Animation` (`self.SleepAnimations`)))
  ;[1 1 1] Set the user-defined sleeping defauts for the player in the loaded sleep data
  (bind _structout (setmembers `/Game/n00dComponents/n00dPacks/n00dGameplay/n00dSleeper/Blueprints/FN00dSleeper_Data` :`StructRef` (`self.LoadedSleepData`) :`Animations` (make `/Game/n00dComponents/n00dPacks/n00dGameplay/n00dSleeper/Blueprints/FN00dSleeper_Animation` _sleepanimations_tosleep _sleepanimations_sleeploop _sleepanimations_fromsleep) :`Sounds` (make `/Game/n00dComponents/n00dPacks/n00dGameplay/n00dSleeper/Blueprints/FN00dSleeper_Sounds` _sleepsounds_tosleep _sleepsounds_sleeploop _sleepsounds_fromsleep)))
  (set `self.LoadedSleepData` _structout)
  (return))

(fn `ControllerInitialise`
  ;[1 1 1] Save the mesh of the owning character in the controller's loaded data, to use on the sleep actor on logout
  (setmembers `/Game/n00dComponents/n00dPacks/n00dGameplay/n00dSleeper/Blueprints/FN00dSleeper_Data` :`StructRef` (`self.LoadedSleepData`) :`SkeletalMesh` (`SkinnedMeshComponent.SkeletalMesh` (`self.OwningSkeletalMesh`)))
  ;[1 1 1] Only do the following for the local
  (if (`Controller.IsLocalController` (`self.OwningController`))
    ;[1 1 1] Set the controller GUID from the instance and fade vision
    (`self.SetControllerGUID` (`self.GetGameInstanceSleepData`))
    (`self.SleepVision`)
    (return)))

(fn `DebugConnectSleeperSession`
  (params (IP_port :type String))
  (`KismetSystemLibrary.ExecuteConsoleCommand` (`KismetStringLibrary.Concat_StrStr` "open " IP_port) (`self.OwningPlayerController`))
  (return))

(fn `DebugOpenSleeperSession`
  (`KismetSystemLibrary.ExecuteConsoleCommand` "open n00dSleeper?listen" (`self.OwningPlayerController`))
  (return))

(fn `DeleteClientSleepData`
  (bind _returnvalue (`GameplayStatics.DoesSaveGameExist` "SleeperSaveClient"))
  (if _returnvalue
    ;[1 1 1] Delete
    (`GameplayStatics.DeleteGameInSlot` "SleeperSaveClient")
    ;[0.2462 0.323 0.34] DEBUG
    (`self.Debug` "Deleted Client Save" "NewEnumerator4")
    (else
      ;[0.2462 0.323 0.34] DEBUG
      (`self.Debug` "Nothing to Delete" "NewEnumerator0"))))

(fn `DeleteServerSleepData`
  (bind _returnvalue (`GameplayStatics.DoesSaveGameExist` (`self.ServerSaveSlot`)))
  (if _returnvalue
    ;[1 1 1] Delete
    (bind _returnvalue_2 (`GameplayStatics.DeleteGameInSlot` (`self.ServerSaveSlot`)))
    ;[0.2462 0.323 0.34] DEBUG
    (`self.Debug` "Deleted Server Save" "NewEnumerator4" (`KismetStringLibrary.Conv_BoolToString` _returnvalue_2))
    (else
      ;[0.2462 0.323 0.34] DEBUG
      (`self.Debug` "Nothing to Delete" "NewEnumerator0"))))

(fn `GameModeInitialise`
  ;[0.09035 0.695 0.1803] Initialise Game Mode Sleeper Component
  ;;[1 1 1] Store a reference to the owner
  (set `self.OwningGameMode` (cast `GameMode` (`self.GetOwner`) :!pure true))
  ;;[1 1 1] LOAD
  ;;;[1 1 1] Load the server save game object
  (`self.LoadServerFromSlot`)
  ;;;[1 1 1] Load the array from the save to an active reference
  (`self.LoadServerSleeperData`)
  ;;;[1 1 1] Load a sleep actor for each sleep data found in the array
  (`self.LoadSleeperActors`)
  (return))

(fn `GetClientSleepData`
  (returns (LoadedSleepData :type "/Game/n00dComponents/n00dPacks/n00dGameplay/n00dSleeper/Blueprints/FN00dSleeper_Data Structure"))
  (return (`self.LoadedSleepData`)))

(fn `GetGameInstanceSleepData`
  (returns (ClientSleepData :type "/Game/n00dComponents/n00dPacks/n00dGameplay/n00dSleeper/Blueprints/FN00dSleeper_Data Structure"))
  ;[1 1 1] We cannot componentise the Game Instance, so we are messaging your Instance for the data
  (bind _sleepdata (message `/Game/n00dComponents/n00dPacks/n00dGameplay/n00dSleeper/Blueprints/BPI_N00dSleeper.GetSleepData` (`GameplayStatics.GetGameInstance`)))
  (return _sleepdata) ; Let's do this
)

(fn `GetServerSleepData`
  (params (ForController :type "Controller Object Reference"))
  (returns (Found :type Boolean) (SleepDataForController :type "/Game/n00dComponents/n00dPacks/n00dGameplay/n00dSleeper/Blueprints/FN00dSleeper_Data Structure"))
  (locals (LocalFound :type Boolean) (LocalSleepData :type "/Game/n00dComponents/n00dPacks/n00dGameplay/n00dSleeper/Blueprints/FN00dSleeper_Data Structure") (LocalControllerGUID :type "Guid Structure"))
  ;[1 1 1] Cache incoming
  (bind _sleepdata (message `/Game/n00dComponents/n00dPacks/n00dGameplay/n00dSleeper/Blueprints/BPI_N00dSleeper.GetSleepData` ForController))
  (set `local.LocalControllerGUID` (`.SleeperGUID_16_625A7DD04788A2F9AC701AA1341AE7EF` (break `/Game/n00dComponents/n00dPacks/n00dGameplay/n00dSleeper/Blueprints/FN00dSleeper_Data` _sleepdata)))
  ;[1 1 1] Loop the game mode loaded server sleep data and find the save associated with the controller
  (bind _sleepercomponent (message `/Game/n00dComponents/n00dPacks/n00dGameplay/n00dSleeper/Blueprints/BPI_N00dSleeper.GetSleeperComponent` (`GameplayStatics.GetGameMode`)))
  (for _array_element (`/Game/n00dComponents/n00dPacks/n00dGameplay/n00dSleeper/Blueprints/BPC_N00dSleeper.LoadedServerSleepData` _sleepercomponent)
    (if (== (`.SleeperGUID_16_625A7DD04788A2F9AC701AA1341AE7EF` (break `/Game/n00dComponents/n00dPacks/n00dGameplay/n00dSleeper/Blueprints/FN00dSleeper_Data` _array_element)) (`local.LocalControllerGUID`))
      (set `local.LocalFound` true)
      (set `local.LocalSleepData` _array_element)))
  ;[1 1 1] Once complete, return with the set values
  (return (`local.LocalFound`) (`local.LocalSleepData`)))

(fn `GetSleepActor`
  (params (ForController :type "Controller Object Reference"))
  (returns (SleepActor :type "/Game/n00dComponents/n00dPacks/n00dGameplay/n00dSleeper/Blueprints/N00dSleeperActor Object Reference"))
  (return (`|GetArrayItem` (`self.ActiveSleepActors`) (+ (`.SleepActorIndex_20_43AFEB9740D88D28FA4A2D80BC7285DA` (break `/Game/n00dComponents/n00dPacks/n00dGameplay/n00dSleeper/Blueprints/FN00dSleeper_Data` (`.SleepDataForController` (`self.GetServerSleepData` ForController)))) 1))))

(fn `GetSleepDataFromServerSave`
  (params (ForController :type "Controller Object Reference"))
  (returns (ServerSleepDataForController :type "/Game/n00dComponents/n00dPacks/n00dGameplay/n00dSleeper/Blueprints/FN00dSleeper_Data Structure") (Found :type Boolean))
  (locals (LocalSleepData :type "Array of /Game/n00dComponents/n00dPacks/n00dGameplay/n00dSleeper/Blueprints/FN00dSleeper_Data Structure") (FoundData :type Boolean) (LocalClient :type "/Game/n00dComponents/n00dPacks/n00dGameplay/n00dSleeper/Blueprints/FN00dSleeper_Data Structure") (LocalServer :type "/Game/n00dComponents/n00dPacks/n00dGameplay/n00dSleeper/Blueprints/FN00dSleeper_Data Structure"))
  (bind _sleepersaveserver (`self.SleeperSaveServer`))
  ;[1 1 1] Get the sleep data from the server save and return it
  (bind _sleepdata (message `/Game/n00dComponents/n00dPacks/n00dGameplay/n00dSleeper/Blueprints/BPI_N00dSleeper.GetSleepData` ForController))
  (set `local.LocalClient` _sleepdata)
  ;[1 1 1] Is the server save valid (always should be, but safety first)
  (`/Engine/EditorBlueprintResources/StandardMacros.IsValid` _sleepersaveserver
    (:`Is Valid`
      ;[1 1 1] If the client is the same as the server, return true
      (for _array_element (`/Game/n00dComponents/n00dPacks/n00dGameplay/n00dSleeper/Blueprints/N00dSleeperSaveServer.SleepData` _sleepersaveserver)
        (if (== (`.SleeperGUID_16_625A7DD04788A2F9AC701AA1341AE7EF` (break `/Game/n00dComponents/n00dPacks/n00dGameplay/n00dSleeper/Blueprints/FN00dSleeper_Data` (`local.LocalClient`))) (`.SleeperGUID_16_625A7DD04788A2F9AC701AA1341AE7EF` (break `/Game/n00dComponents/n00dPacks/n00dGameplay/n00dSleeper/Blueprints/FN00dSleeper_Data` _array_element)))
          (set `local.LocalServer` _array_element)
          (set `local.FoundData` true)))
      (return _array_element (`local.FoundData`)))
    (:`Is Not Valid`
      (return (struct) false))))

(fn `HandleMovement`
  (params (Disable :type Boolean))
  (bind _owningcmc (`self.OwningCMC`))
  (if Disable
    (`CharacterMovementComponent.DisableMovement` _owningcmc)
    (else
      (`CharacterMovementComponent.SetMovementMode` _owningcmc "MOVE_Walking" 0))))

(fn `LoadServerFromSlot`
  (bind _serversaveslot (`self.ServerSaveSlot`))
  (`/Engine/EditorBlueprintResources/StandardMacros.IsValid` (`self.SleeperSaveServer`)
    (:`Is Valid`
      _)
    (:`Is Not Valid`
      ;[1 1 1] If a sleeper save game exists, load it from slot and store a reference to the save game object. If one does not exist on the slot, save to slot
      ;;[1 1 1] Create a sleeper save game object if one does not exist
      (bind _returnvalue (`GameplayStatics.CreateSaveGameObject` "/Game/n00dComponents/n00dPacks/n00dGameplay/n00dSleeper/Blueprints/N00dSleeperSaveServer.N00dSleeperSaveServer_C"))
      (set `self.SleeperSaveServer` _returnvalue)))
  (bind _returnvalue_2 (`GameplayStatics.DoesSaveGameExist` (`self.ServerSaveSlot`)))
  (if _returnvalue_2
    (bind _returnvalue_3 (`GameplayStatics.LoadGameFromSlot` _serversaveslot))
    (bind _asn00d_sleeper_save_server (cast `/Game/n00dComponents/n00dPacks/n00dGameplay/n00dSleeper/Blueprints/N00dSleeperSaveServer` _returnvalue_3))
    (set `self.SleeperSaveServer` _asn00d_sleeper_save_server)
    ;;[0.2462 0.323 0.34] DEBUG
    (`self.Debug` "SAVE LOADED on SERVER" "NewEnumerator0" "" false true 5.0)
    (else
      (bind _returnvalue_4 (`GameplayStatics.SaveGameToSlot` (`self.SleeperSaveServer`) _serversaveslot))
      (if _returnvalue_4
        (`self.Debug` "INITIAL SAVE on the SERVER" "NewEnumerator0" "" false true 5.0)
        (else
          (`self.Debug` "INITIAL SAVE on the SERVER FAILED" "NewEnumerator4" "" false false 5.0))))))

(fn `LoadServerSleeperData`
  ;[1 1 1] Set the loaded from the server save
  (set `self.LoadedServerSleepData` (`/Game/n00dComponents/n00dPacks/n00dGameplay/n00dSleeper/Blueprints/N00dSleeperSaveServer.SleepData` (`self.SleeperSaveServer`)))
  (return))

(fn `LoadSleeperActors`
  (locals (LocalElement :type Integer :default 0) (LocalCount :type Integer))
  ;[1 1 1] Spawn a sleeper actor for each sleep data found on the server
  ;;[1 1 1] Loops the loaded sleep data and grab its location and index
  (for (_array_element _array_index) (`self.LoadedServerSleepData`)
    (set `local.LocalElement` _array_index)
    (bind ((`Sounds_32_0ED13F04442334FEB05781AA7C0F27EC` _sounds) (`SleepActorIndex_20_43AFEB9740D88D28FA4A2D80BC7285DA` _sleepactorindex) (`Location_26_A8C917AB4127A8BA4FB850BA4A5C61D7` _location) (`Rotation_29_9C493C3448359FCDCE17268620ACF414` _rotation)) (break `/Game/n00dComponents/n00dPacks/n00dGameplay/n00dSleeper/Blueprints/FN00dSleeper_Data` _array_element))
    ;;[1 1 1] Spawn the Sleeper Actor per element at the loaded location and rotation
    (bind _returnvalue (`|SpawnActorFromClass` "/Game/n00dComponents/n00dPacks/n00dGameplay/n00dSleeper/Blueprints/N00dSleeperActor.N00dSleeperActor_C" (`KismetMathLibrary.MakeTransform` _location _rotation) "Undefined" "OverrideRootScale" null _array_element))
    ;;[1 1 1] Save these
    (`self.AddToActiveSleeperActors` _returnvalue null (`local.LocalElement`) _sleepactorindex)
    ;;[1 1 1] Increment local Int
    (`/Engine/EditorBlueprintResources/StandardMacros.IncrementInt` (`local.LocalCount`)))
  ;;[0.2462 0.323 0.34] DEBUG
  (`self.Debug` (`KismetStringLibrary.Concat_StrStr` (`KismetStringLibrary.Conv_IntToString` (`local.LocalCount`)) " Sleep Actor(s) Loaded on Server") "NewEnumerator4" "" false true 10.0))

(fn `OnSleeperLogout`
  (params (ExitingController :type "Controller Object Reference"))
  (locals (LocalExiting :type "Controller Object Reference") (LocalServerSleepData :type "/Game/n00dComponents/n00dPacks/n00dGameplay/n00dSleeper/Blueprints/FN00dSleeper_Data Structure"))
  (bind (_found _sleepdataforcontroller) (`self.GetServerSleepData` (`local.LocalExiting`)))
  ;[1 1 1] Handle sleeper logout
  ;;[1 1 1] Add the exiting controller to the server save array
  (set `local.LocalExiting` ExitingController)
  ;;[1 1 1] Check if the server has a save for this controller
  (if _found
    ;;[1 1 1] Store the server as a local
    (set `local.LocalServerSleepData` _sleepdataforcontroller)
    (else
      ;;[1 1 1] If there is none found, store the local from the controller
      (bind _sleepdata (message `/Game/n00dComponents/n00dPacks/n00dGameplay/n00dSleeper/Blueprints/BPI_N00dSleeper.GetSleepData` (`local.LocalExiting`)))
      (set `local.LocalServerSleepData` _sleepdata)
      ;;[1 1 1] Add the exiting player to the server array
      (`self.AddPlayerToSleeperArray` (`local.LocalExiting`))))
  ;;[1 1 1] Spawn the sleep actor and handle actor information
  ;;;[1 1 1] Spawn the sleeper actor in the world at the player's location and with the controller's sleep data
  (bind _sleepactor (`self.SpawnSleepActor` (`local.LocalExiting`)))
  ;;;[1 1 1] Get the current information from the controller and parse it to the spawned sleep actor
  (bind _sleepdata_2 (message `/Game/n00dComponents/n00dPacks/n00dGameplay/n00dSleeper/Blueprints/BPI_N00dSleeper.GetSleepData` (`local.LocalExiting`)))
  (`/Game/n00dComponents/n00dPacks/n00dGameplay/n00dSleeper/Blueprints/N00dSleeperActor.FallAsleep` _sleepactor _sleepdata_2)
  ;;;[0.2462 0.323 0.34] DEBUG
  (`self.Debug` "Spawned Sleep Actor:" "NewEnumerator2" (`KismetSystemLibrary.GetDisplayName` _sleepactor))
  (return))

(fn `OnSleeperPostLogin`
  (params (NewController :type "Controller Object Reference"))
  (locals (LocalController :type "Controller Object Reference") (LocalClientGUID :type "Guid Structure") (LocalServerGUID :type "Guid Structure") (LocalLocation :type "Vector Structure") (LocalRotation :type "Rotator Structure") (LocalActorIndex :type Integer) (LocalServerSleepData :type "/Game/n00dComponents/n00dPacks/n00dGameplay/n00dSleeper/Blueprints/FN00dSleeper_Data Structure") (LocalControllerSleepActor :type "/Game/n00dComponents/n00dPacks/n00dGameplay/n00dSleeper/Blueprints/N00dSleeperActor Object Reference"))
  (bind (_found _sleepdataforcontroller) (`self.GetServerSleepData` (`local.LocalController`)))
  ;[1 1 1] Post Login
  ;;[1 1 1] Cache
  (set `local.LocalController` NewController)
  ;;[1 1 1] Get the GUID for controller from the server
  (if (`self.GetServerSleepData` (`local.LocalController`))
    ;;[1 1 1] Is the GUID valid, in case we've saved an invalid reference
    (if (`KismetGuidLibrary.IsValid_Guid` (`.SleeperGUID_16_625A7DD04788A2F9AC701AA1341AE7EF` (break `/Game/n00dComponents/n00dPacks/n00dGameplay/n00dSleeper/Blueprints/FN00dSleeper_Data` _sleepdataforcontroller)))
      (set `local.LocalServerSleepData` _sleepdataforcontroller) ; Store the SleepData as a local
      ;;[0.2462 0.323 0.34] DEBUG
      ;;;[1 1 1] Set the sleeper GUID from server as an owner value for debug
      (message `/Game/n00dComponents/n00dPacks/n00dGameplay/n00dSleeper/Blueprints/BPI_N00dSleeper.SetSleepData` (`local.LocalController`) (`local.LocalServerSleepData`)) ; Set the debug sleep data on the controller
      ;;[1 1 1] Get the controller's sleep data
      (bind _sleepdata (message `/Game/n00dComponents/n00dPacks/n00dGameplay/n00dSleeper/Blueprints/BPI_N00dSleeper.GetSleepData` (`local.LocalController`)))
      ;;[1 1 1] Loop the active sleep actors and find the one that matches the player's GUID
      (for _array_element (`self.ActiveSleepActors`)
        (if (== (`.SleeperGUID_16_625A7DD04788A2F9AC701AA1341AE7EF` (break `/Game/n00dComponents/n00dPacks/n00dGameplay/n00dSleeper/Blueprints/FN00dSleeper_Data` (`/Game/n00dComponents/n00dPacks/n00dGameplay/n00dSleeper/Blueprints/N00dSleeperActor.SleepData` _array_element))) (`.SleeperGUID_16_625A7DD04788A2F9AC701AA1341AE7EF` (break `/Game/n00dComponents/n00dPacks/n00dGameplay/n00dSleeper/Blueprints/FN00dSleeper_Data` _sleepdata)))
          (set `local.LocalControllerSleepActor` _array_element)
          ;;[1 1 1] @TODO don't do on initial load
          ;;;[1 1 1] Wake up
          (`/Game/n00dComponents/n00dPacks/n00dGameplay/n00dSleeper/Blueprints/N00dSleeperActor.WakeUp` (`local.LocalControllerSleepActor`) (`local.LocalController`))))
      (else
        ;;[0.2462 0.323 0.34] DEBUG
        (`self.Debug` "Server Sleep Data INVALID" "NewEnumerator4")
        (return)))
    (else
      ;;;[1 1 1] DEBUG
      (`self.Debug` "SERVER SAVE for CONTROLLER NOT FOUND - Is this your first log in attempt, or have you defined the correct Game Instance in the Project Settings" "NewEnumerator4" "" false false 20.0))))

(fn `RemovePlayerFromSleeperArray`
  (params (ForController :type "Controller Object Reference"))
  ;[1 1 1] Get controller sleep data and remove it from the server array, then save
  (bind _sleepdata (message `/Game/n00dComponents/n00dPacks/n00dGameplay/n00dSleeper/Blueprints/BPI_N00dSleeper.GetSleepData` ForController))
  (`KismetArrayLibrary.Array_RemoveItem` (`self.LoadedServerSleepData`) _sleepdata)
  (`self.SaveLoadedServerSleeperData`)
  (return))

(fn `RemoveSleepActor`
  (params (SleepActorToRemove :type "/Game/n00dComponents/n00dPacks/n00dGameplay/n00dSleeper/Blueprints/N00dSleeperActor Object Reference"))
  (locals (LocalSleepActor :type "/Game/n00dComponents/n00dPacks/n00dGameplay/n00dSleeper/Blueprints/N00dSleeperActor Object Reference"))
  (bind _localsleepactor (`local.LocalSleepActor`))
  ;[1 1 1] Handle the sleeper actor
  ;;[1 1 1] Cache
  (set `local.LocalSleepActor` SleepActorToRemove)
  ;;[0.2462 0.323 0.34] DEBUG
  (`self.Debug` (`KismetStringLibrary.Concat_StrStr` "REMOVED SLEEP ACTOR: " (`KismetSystemLibrary.GetDisplayName` _localsleepactor) " on INDEX: " (`KismetStringLibrary.Conv_IntToString` (`KismetArrayLibrary.Array_Find` (`self.ActiveSleepActors`) _localsleepactor))) "NewEnumerator4" "" false true 5.0)
  ;;[1 1 1] Remove the incoming from the array
  (`KismetArrayLibrary.Array_RemoveItem` (`self.ActiveSleepActors`) (`local.LocalSleepActor`))
  ;;[1 1 1] Destroy it and return
  (`Actor.K2_DestroyActor` (`local.LocalSleepActor`))
  (return))

(fn `ResolveSleeperWorldPositioning`
  (params (Sleeper :type "Actor Object Reference"))
  (returns (Location :type "Vector Structure") (Yaw :type "Float (double-precision)"))
  (bind (_returnvalue_roll _returnvalue_pitch _returnvalue_yaw) (`KismetMathLibrary.BreakRotator` (`Actor.K2_GetActorRotation` Sleeper)))
  (return (`Actor.K2_GetActorLocation` Sleeper) _returnvalue_yaw))

(fn `SaveLoadedServerSleeperData`
  ;[1 1 1] Grab the loaded game mode SleepData and save it to the save object
  (set `/Game/n00dComponents/n00dPacks/n00dGameplay/n00dSleeper/Blueprints/N00dSleeperSaveServer.SleepData` (`self.LoadedServerSleepData`) (`self.SleeperSaveServer`))
  (`self.SaveServerToSlot`)
  (return))

(fn `SaveServerToSlot`
  (returns (ReturnValue :type Boolean))
  ;[1 1 1] Save the server to slot
  (bind _returnvalue (`GameplayStatics.SaveGameToSlot` (`self.SleeperSaveServer`) (`self.ServerSaveSlot`)))
  (if _returnvalue
    (`self.Debug` "Server SUCCEEDED in Saving Game to Slot" "NewEnumerator0")
    (else
      (`self.Debug` "Server FAILED to Save Game to Slot" "NewEnumerator4")))
  (return _returnvalue))

(fn `SetControllerGUID`
  (params (SleepData :type "/Game/n00dComponents/n00dPacks/n00dGameplay/n00dSleeper/Blueprints/FN00dSleeper_Data Structure (by ref)"))
  ;[1 1 1] Controller stores client GUID
  ;;[1 1 1] Set the client sleeper GUID on the controller from the instance, on controller initialise as we need it in game mode PostLogin.
  (bind _structout (setmembers `/Game/n00dComponents/n00dPacks/n00dGameplay/n00dSleeper/Blueprints/FN00dSleeper_Data` :`StructRef` (`self.LoadedSleepData`) :`SleeperGUID` (`.SleeperGUID_16_625A7DD04788A2F9AC701AA1341AE7EF` (break `/Game/n00dComponents/n00dPacks/n00dGameplay/n00dSleeper/Blueprints/FN00dSleeper_Data` SleepData))))
  (`self.SetControllerSleepData` _structout)
  (return))

(fn `SetControllerSleepData`
  (params (SleepData :type "/Game/n00dComponents/n00dPacks/n00dGameplay/n00dSleeper/Blueprints/FN00dSleeper_Data Structure"))
  ;[1 1 1] Set the component sleep data to represent the Client load from instance
  ;;[1 1 1] Set the members in the sleeper data with info from the component
  (bind _output_get (set `self.LoadedSleepData` SleepData))
  (`self.ServerSetLoadedSleepData` _output_get)
  ;;[1 1 1] DEBUG
  (`self.Debug` "SET LOADED SleepData for Controller GUID:" "NewEnumerator2" (`KismetGuidLibrary.Conv_GuidToString` (`.SleeperGUID_16_625A7DD04788A2F9AC701AA1341AE7EF` (break `/Game/n00dComponents/n00dPacks/n00dGameplay/n00dSleeper/Blueprints/FN00dSleeper_Data` _output_get))) false true 10.0)
  (return))

(fn `SetControllerSleepDataGUID`
  (params (SleeperGUID :type "Guid Structure"))
  ;[1 1 1] Set the sleeper data GUID
  (`self.ControllerHasAuthority`
    (:`Authority`
      (bind _structout (setmembers `/Game/n00dComponents/n00dPacks/n00dGameplay/n00dSleeper/Blueprints/FN00dSleeper_Data` :`StructRef` (`self.LoadedSleepData`) :`SleeperGUID` SleeperGUID))
      (`self.SetControllerSleepData` _structout)
      ;[0.2462 0.323 0.34] DEBUG
      (`self.Debug` "Controller GUID" "NewEnumerator2" (`KismetGuidLibrary.Conv_GuidToString` (`.SleeperGUID_16_625A7DD04788A2F9AC701AA1341AE7EF` (break `/Game/n00dComponents/n00dPacks/n00dGameplay/n00dSleeper/Blueprints/FN00dSleeper_Data` (`self.LoadedSleepData`)))) false true 5.0)
      (return))
    (:`Remote`
      (`self.ServerSetSleeperGUID` SleeperGUID))))

(fn `SleepVision`
  ;[1 1 1] Set the camera manager's camera fade function and a custom timer informing when to start fade
  (if (`self.UseScreenFade`)
    (`PlayerCameraManager.SetManualCameraFade` :`self` (`PlayerController.PlayerCameraManager` (`GameplayStatics.GetPlayerController` 0)) :`InFadeAmount` 1.0)
    (`KismetSystemLibrary.K2_SetTimer` null "SleepVisionTimer" (`self.SleepVisionFadeDelay`))
    (return)
    (else
      (return))))

(fn `SleepVisionTimer`
  ;[1 1 1] This will always be fired from the remote, so we can use get player character here
  (`PlayerCameraManager.StartCameraFade` :`self` (`PlayerController.PlayerCameraManager` (`GameplayStatics.GetPlayerController` 0)) :`FromAlpha` 1.0 :`Duration` (- (`AnimSequenceBase.SequenceLength` (`.FromSleep_6_BE4A8AAA4058BC40F7E3B995B7FC0BD9` (break `/Game/n00dComponents/n00dPacks/n00dGameplay/n00dSleeper/Blueprints/FN00dSleeper_Animation` (`.Animations_23_0C71528045C90A61DD4D64B48A4F1F75` (break `/Game/n00dComponents/n00dPacks/n00dGameplay/n00dSleeper/Blueprints/FN00dSleeper_Data` (`self.LoadedSleepData`)))))) (`self.SleepVisionFadeDelay`)))
  (return))

(fn `SpawnSleepActor`
  (params (ForController :type "Controller Object Reference"))
  (returns (SleepActor :type "/Game/n00dComponents/n00dPacks/n00dGameplay/n00dSleeper/Blueprints/N00dSleeperActor Object Reference"))
  (locals (LocalController :type "Controller Object Reference"))
  (bind _localcontroller (`local.LocalController`))
  (bind (_location _yaw) (`self.ResolveSleeperWorldPositioning` (`local.LocalController`)))
  ;[1 1 1] Spawn the sleep actor and set the owner SleepData in the recently spawned actor - add them to an array to call on later, such as logon
  (bind _output_get (set `local.LocalController` ForController))
  (bind _sleepdata (message `/Game/n00dComponents/n00dPacks/n00dGameplay/n00dSleeper/Blueprints/BPI_N00dSleeper.GetSleepData` _output_get))
  (bind _returnvalue (`|SpawnActorFromClass` "/Game/n00dComponents/n00dPacks/n00dGameplay/n00dSleeper/Blueprints/N00dSleeperActor.N00dSleeperActor_C" (`KismetMathLibrary.MakeTransform` _location (`KismetMathLibrary.MakeRotator` 0.0 0.0 _yaw)) "AdjustIfPossibleButAlwaysSpawn" "OverrideRootScale" _localcontroller _sleepdata _localcontroller (`Actor.Instigator` _localcontroller)))
  ;;[0.2462 0.323 0.34] DEBUG
  (`self.Debug` "SLEEP ACTOR LOCATION: " "NewEnumerator2" (`KismetStringLibrary.Conv_VectorToString` _location) false true 10.0)
  ;;[1 1 1] Add the spawned sleep actor to an array
  (bind _output_get_2 (set `self.SleepActor` _returnvalue))
  (`self.AddToActiveSleeperActors` _output_get_2 (`local.LocalController`))
  (return _output_get_2))